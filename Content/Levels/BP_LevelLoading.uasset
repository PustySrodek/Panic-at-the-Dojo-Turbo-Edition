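; BP_LevelLoading is a Blueprint that switches between streaming levels, tracking one loaded level by name.
; LoadLevel acts only when the requested name differs from LoadedLevel or Force is set.
; It flags the previous streaming level to unload and hide, stores the new name, and flags that level to load and become visible.
; An unresolvable name prints an error unless it is "None".
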(fn `Load Level`
  (params (Level :type String) (Force :type Boolean))
  (bind _returnvalue (`GameplayStatics.GetStreamingLevel` (`KismetStringLibrary.Conv_StringToName` (`self.Loaded Level`))))
  (if (or Force (`KismetStringLibrary.NotEqual_StrStr` (`local.Level`) (`self.Loaded Level`)))
    (`|ExecutionSequence`
      (:`then_0`
        (`/Engine/EditorBlueprintResources/StandardMacros.IsValid` _returnvalue
          (:`Is Valid`
            (set `LevelStreaming.bShouldBeLoaded` false _returnvalue)
            (set `LevelStreaming.bShouldBeVisible` false _returnvalue))))
      (:`then_1`
        (bind _output_get (set `self.Loaded Level` (`local.Level`)))
        (bind _returnvalue_2 (`GameplayStatics.GetStreamingLevel` (`KismetStringLibrary.Conv_StringToName` _output_get)))
        (`/Engine/EditorBlueprintResources/StandardMacros.IsValid` _returnvalue_2
          (:`Is Valid`
            (set `LevelStreaming.bShouldBeLoaded` true _returnvalue_2)
            (set `LevelStreaming.bShouldBeVisible` true _returnvalue_2))
          (:`Is Not Valid`
            (if (not (`KismetStringLibrary.EqualEqual_StrStr` (`self.Loaded Level`)))
              (`KismetSystemLibrary.PrintString` (`KismetStringLibrary.Concat_StrStr` "Load Level Function Error. Invalid Level Name: " "\"" (`self.Loaded Level`) "\"") true true (struct :`R` 0.645833 :`A` 1.0) 5.0))))))))

(fn `UserConstructionScript`)