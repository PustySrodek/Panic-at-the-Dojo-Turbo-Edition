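; BP_Pathfinding runs A* searches over GridRef's square or hex grid, returning either a path to a target or tiles reachable within PathLength.
; Neighbours are filtered by tile type, occupying unit and height, with tile and obstacle costs.
; A cost-sorted open list favours straight steps over diagonals on ties.
; Searches run instantly or step through a retriggerable delay, firing update and completion callbacks.
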(event `FindPathWithDelay`
  (`|ExecutionSequence`
    (:`then_0`
      (goto _label_3 :!via `Open`))
    (:`then_1`
      (set `self.Loop Start Time` (`KismetMathLibrary.Now`) :!label _label)
      (if (> (`KismetArrayLibrary.Array_Length` (`self.Discovered Tiles`)) 0)
        (bind _found_target (`self.Analyze Next Discovered Tile`))
        (if _found_target :!label _label_2
          (bind _path (`self.Generate Path`))
          (`self.On Pathfinding Completed` _path)
          (else
            (if (> (`self.MaxMsPerFrame`) 0.0)
              (if (> (`KismetMathLibrary.GetTotalMilliseconds` (- (`KismetMathLibrary.Now`) (`self.Loop Start Time`))) (`self.MaxMsPerFrame`))
                (goto _label_2)
                (else
                  _)))
            (`KismetSystemLibrary.RetriggerableDelay` (`self.Delay`))
            (`/Engine/EditorBlueprintResources/StandardMacros.Gate` true :!label _label_3
              (:`Exit`
                (goto _label)))))
        (else
          (`self.On Pathfinding Completed` (select `bool` (`self.Generate Reachable`) :`false` (`|MakeArray`) :`true` (`self.Analysed Tiles`))))))))

(event `Close Delay Gate`
  (goto _label_3 :!via `Close`))

(fn `Analyze Next Discovered Tile`
  (returns (`Found Target` :type Boolean))
  (bind _cheapest_tile (`self.Pull the Cheapest`))
  (bind _output_get (set `self.Current Discovered Tile` _cheapest_tile))
  (`self.On Pathfinding Data Updated` (`.Index_4_9BE497C941A7AA9C40E42F8D48724B12` (break `/Game/Blueprints/Grid/F_PathfindingData` _output_get)))
  (bind _neighnours (`self.Get Valid Neighbours` (`.Index_4_9BE497C941A7AA9C40E42F8D48724B12` (break `/Game/Blueprints/Grid/F_PathfindingData` _output_get)) (`self.Use Diagonals`) (`self.Valid Types`)))
  (bind _output_get_2 (set `self.Current Neighnours` _neighnours))
  (while (> (`KismetArrayLibrary.Array_Length` _output_get_2) 0)
    (bind _is_target_tile (`self.Discover Next Neighbour`))
    (if _is_target_tile
      (return true)))
  (return false))

(fn `Clear Data`
  (`|ExecutionSequence`
    (:`then_0`
      (`KismetArrayLibrary.Array_Clear` (`self.Analysed Tiles`)))
    (:`then_1`
      (`KismetArrayLibrary.Array_Clear` (`self.Discovered Tiles`)))
    (:`then_2`
      (`KismetArrayLibrary.Array_Clear` (`self.Discovered Tile Sorting Cost`)))
    (:`then_3`
      (`BlueprintMapLibrary.Map_Clear` (`self.Pathfinding Data`)))
    (:`then_4`
      (`self.On Pathfinding Data Cleared`))))

(fn `Discover Next Neighbour`
  (returns (`Is Target Tile` :type Boolean))
  (locals (`Cost From Start` :type Integer) (`Index in Discovered` :type Integer :default 0))
  (bind _index_in_discovered (`local.Index in Discovered`))
  (bind (_index _previousindex _costtoentertile) (break `/Game/Blueprints/Grid/F_PathfindingData` (`self.Current Neighnour`)))
  (set `self.Current Neighnour` (`|GetArrayItem` (`self.Current Neighnours`)))
  (`KismetArrayLibrary.Array_Remove` (`self.Current Neighnours`))
  (if (not (`KismetArrayLibrary.Array_Contains` (`self.Analysed Tiles`) (`.Index_4_9BE497C941A7AA9C40E42F8D48724B12` (break `/Game/Blueprints/Grid/F_PathfindingData` (`self.Current Neighnour`)))))
    (set `local.Cost From Start` (+ (`.CostToEnterTile_10_CD261BB54EAC367A21D2509DC1B718BB` (break `/Game/Blueprints/Grid/F_PathfindingData` (`self.Current Neighnour`))) (`.CostFromtheStart_13_E64E351248D244B4BB5C4B8B3BE2AB1C` (break `/Game/Blueprints/Grid/F_PathfindingData` (`self.Current Discovered Tile`)))))
    (if (<= (`local.Cost From Start`) (`self.Path Length`))
      (bind _output_get (set `local.Index in Discovered` (`KismetArrayLibrary.Array_Find` (`self.Discovered Tiles`) (`.Index_4_9BE497C941A7AA9C40E42F8D48724B12` (break `/Game/Blueprints/Grid/F_PathfindingData` (`self.Current Neighnour`))))))
      (if (not (== _output_get -1))
        (bind _output_get_2 (set `self.Current Neighnour` (`BlueprintMapLibrary.Map_Find` (`self.Pathfinding Data`) (`.Index_4_9BE497C941A7AA9C40E42F8D48724B12` (break `/Game/Blueprints/Grid/F_PathfindingData` (`self.Current Neighnour`))))))
        (if (< (`local.Cost From Start`) (`.CostFromtheStart_13_E64E351248D244B4BB5C4B8B3BE2AB1C` (break `/Game/Blueprints/Grid/F_PathfindingData` _output_get_2)))
          (`KismetArrayLibrary.Array_Remove` (`self.Discovered Tiles`) _index_in_discovered)
          (`KismetArrayLibrary.Array_Remove` (`self.Discovered Tile Sorting Cost`) _index_in_discovered)
          (else
            (return false))))
      (`self.Discover Tile` (make `/Game/Blueprints/Grid/F_PathfindingData` _index (`.Index_4_9BE497C941A7AA9C40E42F8D48724B12` (break `/Game/Blueprints/Grid/F_PathfindingData` (`self.Current Discovered Tile`))) _costtoentertile (`local.Cost From Start`) (`self.Get Minimal Cost` (`.Index_4_9BE497C941A7AA9C40E42F8D48724B12` (break `/Game/Blueprints/Grid/F_PathfindingData` (`self.Current Neighnour`))) (`self.Target Index`) (`self.Use Diagonals`))))
      (if (`KismetMathLibrary.Equal_IntPointIntPoint` (`.Index_4_9BE497C941A7AA9C40E42F8D48724B12` (break `/Game/Blueprints/Grid/F_PathfindingData` (`self.Current Neighnour`))) (`self.Target Index`))
        (return true)
        (else
          (return false))))
    (else
      (return false))))

(fn `Discover Tile`
  (params (`Tile Path Data` :type "/Game/Blueprints/Grid/F_PathfindingData Structure"))
  (bind _index (break `/Game/Blueprints/Grid/F_PathfindingData` `Tile Path Data`))
  (`BlueprintMapLibrary.Map_Add` (`self.Pathfinding Data`) _index `Tile Path Data`)
  (`self.Inesrt To And Sort Discovered Array` `Tile Path Data`)
  (`self.On Pathfinding Data Updated` _index))

(fn `Find Path`
  (params (`Use Diagonals` :type Boolean) (`Start ` :type "IntPoint Structure") (Target :type "IntPoint Structure") (Delay :type "Float (double-precision)") (MaxMsPerFrame :type "Float (double-precision)") (`Valid Types` :type "Array of /Game/Blueprints/Grid/Obstacles/Enum_TileTypes Enum") (`Generate reachable` :type Boolean) (`Path length` :type Integer))
  (returns (Path :type "Array of IntPoint Structure"))
  (bind _array (`|MakeArray`))
  (bind _returnvalue (select `bool` (`self.Generate Reachable`) :`false` (`|MakeArray`) :`true` (`self.Analysed Tiles`)))
  (set `self.Use Diagonals` `Use Diagonals`)
  (set `self.Start Index` `Start `)
  (set `self.Target Index` Target)
  (set `self.Delay` Delay)
  (set `self.MaxMsPerFrame` MaxMsPerFrame)
  (set `self.Valid Types` `Valid Types`)
  (set `self.Generate Reachable` `Generate reachable`)
  (set `self.Path Length` `Path length`)
  (`self.Close Delay Gate`)
  (`self.Clear Data`)
  (bind _is_valid (`self.Is Input Data Valid`))
  (if _is_valid
    (`self.Discover Tile` (make `/Game/Blueprints/Grid/F_PathfindingData` (`self.Start Index`) (struct :`X` -999 :`Y` -999) 1 0 (`self.Get Minimal Cost` (`self.Start Index`) (`self.Target Index`) (`self.Use Diagonals`))))
    (if (<= (`local.Delay`) 0.0)
      (while (> (`KismetArrayLibrary.Array_Length` (`self.Discovered Tiles`)) 0)
        (bind _found_target (`self.Analyze Next Discovered Tile`))
        (if _found_target
          (bind _path (`self.Generate Path`))
          (`self.On Pathfinding Completed` _path)
          (return _path)))
      (`self.On Pathfinding Completed` _returnvalue)
      (return _returnvalue)
      (else
        (`self.FindPathWithDelay`)
        (return (`|MakeArray`))))
    (else
      (`self.On Pathfinding Completed` _array)
      (return _array))))

(fn `Generate Path`
  (returns (Path :type "Array of IntPoint Structure"))
  (locals (Current :type "IntPoint Structure") (`Inverted Path` :type "Array of IntPoint Structure") (`Correct Path` :type "Array of IntPoint Structure"))
  (bind _output_get (set `local.Current` (`self.Target Index`)))
  (while (!= _output_get (`self.Start Index`))
    (`KismetArrayLibrary.Array_Add` (`local.Inverted Path`) (`local.Current`))
    (set `local.Current` (`.PreviousIndex_6_98BE5378423C2D86947E9D9DF104DF36` (break `/Game/Blueprints/Grid/F_PathfindingData` (`BlueprintMapLibrary.Map_Find` (`self.Pathfinding Data`) (`local.Current`))))))
  (bind (_arrayindex _arrayelement) (`/Engine/EditorBlueprintResources/StandardMacros.ReverseForEachLoop` (`local.Inverted Path`))
    (:`LoopBody`
      (`KismetArrayLibrary.Array_Add` (`local.Correct Path`) _arrayelement))
    (:`Completed`
      (return (`local.Correct Path`)))))

(fn `Get Minimal Cost`
  (params (`Index 1` :type "IntPoint Structure") (`Index 2` :type "IntPoint Structure") (`Use Diagonals` :type Boolean))
  (returns (`Minimal cost` :type Integer))
  (bind (_returnvalue_x _returnvalue_y) (break `IntPoint` (- (`local.Index 1`) (`local.Index 2`))))
  (bind (_returnvalue_x_2 _returnvalue_y_2) (break `IntPoint` (- (`local.Index 1`) (`local.Index 2`))))
  (bind (_returnvalue_x_3 _returnvalue_y_3) (break `IntPoint` (- (`local.Index 1`) (`local.Index 2`))))
  (bind _returnvalue (`KismetMathLibrary.Abs_Int` _returnvalue_x_2))
  (switch `/Game/Blueprints/Grid/Enum_GridShapeData` (`/Game/Blueprints/Grid/BP_Grid.Tile Shape` (`self.Grid Ref`))
    (:`NewEnumerator1`
      (if (`local.Use Diagonals`)
        (return (`KismetMathLibrary.Max` (`KismetMathLibrary.Abs_Int` _returnvalue_x_3) (`KismetMathLibrary.Abs_Int` _returnvalue_y_3)))
        (else
          (return (+ (`KismetMathLibrary.Abs_Int` _returnvalue_x) (`KismetMathLibrary.Abs_Int` _returnvalue_y))))))
    (:`NewEnumerator2`
      (return (+ _returnvalue (`KismetMathLibrary.Max` (/ (- (`KismetMathLibrary.Abs_Int` _returnvalue_y_2) _returnvalue) 2)))))))

(fn `Get N Index Hexagons`
  (params (Index :type "IntPoint Structure"))
  (returns (`Square N Indexes` :type "Array of IntPoint Structure"))
  (locals (Ret :type "Array of IntPoint Structure"))
  (return (`|MakeArray` (+ Index (make `IntPoint` -1 1)) (+ Index (make `IntPoint` 1 -1)) (+ Index (make `IntPoint` 1 1)) (+ Index (make `IntPoint` -1 -1)) (+ Index (make `IntPoint` 0 2)) (+ Index (make `IntPoint` 0 -2)))))

(fn `Get N Index Square`
  (params (Index :type "IntPoint Structure") (`Include Diagonals` :type Boolean))
  (returns (`Square N Indexes` :type "Array of IntPoint Structure"))
  (locals (Ret :type "Array of IntPoint Structure"))
  (bind _array (`|MakeArray` (+ Index (make `IntPoint` 1)) (+ Index (make `IntPoint` 0 1)) (+ Index (make `IntPoint` -1)) (+ Index (make `IntPoint` 0 -1))))
  (if (`local.Include Diagonals`)
    (bind _output_get (set `local.Ret` _array))
    (`KismetArrayLibrary.Array_Append` _output_get (`|MakeArray` (+ Index (make `IntPoint` 1 1)) (+ Index (make `IntPoint` -1 -1)) (+ Index (make `IntPoint` -1 1)) (+ Index (make `IntPoint` 1 -1))))
    (return (`local.Ret`))
    (else
      (return _array))))

(fn `Get Neighbour Indexes`
  (params (Index :type "IntPoint Structure") (`Include Diagonals` :type Boolean))
  (returns (`Vaild Neighbours` :type "Array of IntPoint Structure"))
  (switch `/Game/Blueprints/Grid/Enum_GridShapeData` (`/Game/Blueprints/Grid/BP_Grid.Tile Shape` (`self.Grid Ref`))
    (:`NewEnumerator1`
      (return (`self.Get N Index Square` (`local.Index`) `Include Diagonals`)))
    (:`NewEnumerator2`
      (return (`self.Get N Index Hexagons` (`local.Index`))))))

(fn `Get Path Cost`
  (params (Path :type "Array of IntPoint Structure"))
  (returns (Cost :type Integer))
  (locals (Ret :type Integer))
  (set `local.Ret` 0)
  (for _ (`local.Path`)
    (set `local.Ret` (+ (`local.Ret`) 1)))
  (return (`local.Ret`)))

(fn `Get Valid Neighbours`
  (params (Index :type "IntPoint Structure") (`Include Diagonals` :type Boolean) (`Valid Types` :type "Array of /Game/Blueprints/Grid/Obstacles/Enum_TileTypes Enum"))
  (returns (Neighnours :type "Array of /Game/Blueprints/Grid/F_PathfindingData Structure"))
  (locals (Data :type "/Game/Blueprints/Grid/F_TileData Structure") (`Input Data` :type "/Game/Blueprints/Grid/F_TileData Structure") (`Return Data` :type "Array of /Game/Blueprints/Grid/F_PathfindingData Structure"))
  (bind (_index _tiletype _tiletransform _tilestate _unitontile _obstacles) (break `/Game/Blueprints/Grid/F_TileData` (`local.Data`)))
  (bind (_tile_size_x _tile_size_y _tile_size_z) (`KismetMathLibrary.BreakVector` (`/Game/Blueprints/Grid/BP_Grid.Tile Size` (`self.Grid Ref`))))
  (set `local.Input Data` (`BlueprintMapLibrary.Map_Find` (`/Game/Blueprints/Grid/BP_Grid.Grid Tiles Data` (`self.Grid Ref`)) Index))
  (bind _vaild_neighbours (`self.Get Neighbour Indexes` Index `Include Diagonals`))
  (for _array_element _vaild_neighbours
    (bind _output_get (set `local.Data` (`BlueprintMapLibrary.Map_Find` (`/Game/Blueprints/Grid/BP_Grid.Grid Tiles Data` (`self.Grid Ref`)) _array_element)))
    (if (`KismetArrayLibrary.Array_Contains` (`local.Valid Types`) (`.TileType_7_99A5401643D0FD504FC2D2B4806678DB` (break `/Game/Blueprints/Grid/F_TileData` _output_get)))
      (if (not (`KismetSystemLibrary.IsValid` (`.UnitonTile_19_090F5A1342BB3758B627C38D844712AB` (break `/Game/Blueprints/Grid/F_TileData` (`local.Data`)))))
        (if (<= (`KismetMathLibrary.Abs` (- (.z (.location (`.TileTransform_9_C8B49F424080CB25DC8191A7EE85CF00` (break `/Game/Blueprints/Grid/F_TileData` (`local.Data`))))) (.z (.scale (`.TileTransform_9_C8B49F424080CB25DC8191A7EE85CF00` (break `/Game/Blueprints/Grid/F_TileData` (`local.Input Data`))))))) _tile_size_z)
          (`KismetArrayLibrary.Array_Add` (`local.Return Data`) (make `/Game/Blueprints/Grid/F_PathfindingData` _index (`local.Index`) (+ (`/Game/Blueprints/Core/Utility/BPFL_Utility.Get Tile Type Cost` _tiletype) (select `bool` (`BlueprintMapLibrary.Map_Contains` _obstacles "NewEnumerator12") :`true` 2))))))))
  (return (`local.Return Data`)))

(fn `Inesrt To And Sort Discovered Array`
  (params (`Pathfinding DAta` :type "/Game/Blueprints/Grid/F_PathfindingData Structure"))
  (locals (`Sorting Cost` :type Integer))
  (bind _discovered_tile_sorting_cost (`self.Discovered Tile Sorting Cost`))
  (set `local.Sorting Cost` (`self.Set Priority for Diagonals` `Pathfinding DAta`))
  (if (== (`KismetArrayLibrary.Array_Length` (`self.Discovered Tile Sorting Cost`)) 0)
    (`KismetArrayLibrary.Array_Add` (`self.Discovered Tile Sorting Cost`) (`local.Sorting Cost`) :!label _label)
    (`KismetArrayLibrary.Array_Add` (`self.Discovered Tiles`) (`.Index_4_9BE497C941A7AA9C40E42F8D48724B12` (break `/Game/Blueprints/Grid/F_PathfindingData` (`local.Pathfinding DAta`))))
    (elif (>= (`local.Sorting Cost`) (`|GetArrayItem` _discovered_tile_sorting_cost (`KismetArrayLibrary.Array_LastIndex` _discovered_tile_sorting_cost)))
      (goto _label)
      (else
        (for (_array_element _array_index) (`self.Discovered Tile Sorting Cost`)
          (if (>= _array_element (`local.Sorting Cost`))
            (`KismetArrayLibrary.Array_Insert` (`self.Discovered Tile Sorting Cost`) (`local.Sorting Cost`) _array_index)
            (`KismetArrayLibrary.Array_Insert` (`self.Discovered Tiles`) (`.Index_4_9BE497C941A7AA9C40E42F8D48724B12` (break `/Game/Blueprints/Grid/F_PathfindingData` (`local.Pathfinding DAta`))) _array_index)
            (break)))))))

(fn `Is Diagonal`
  (params (`Index 1` :type "IntPoint Structure") (`Index 2` :type "IntPoint Structure"))
  (returns (`Is Diagonal` :type Boolean))
  (bind _vaild_neighbours (`self.Get Neighbour Indexes` `Index 1`))
  (return (not (`KismetArrayLibrary.Array_Contains` _vaild_neighbours `Index 2`))))

(fn `Is Input Data Valid`
  (returns (`Is Valid` :type Boolean))
  (bind (_index _tiletype _tiletransform _tilestate _unitontile) (break `/Game/Blueprints/Grid/F_TileData` (`BlueprintMapLibrary.Map_Find` (`/Game/Blueprints/Grid/BP_Grid.Grid Tiles Data` (`self.Grid Ref`)) (`self.Target Index`))))
  (if (!= (`self.Start Index`) (`self.Target Index`))
    (if (`/Game/Blueprints/Grid/BP_Grid.Is Tile Walkable` (`self.Grid Ref`) (`self.Start Index`))
      (if (not (`self.Generate Reachable`))
        (if (`/Game/Blueprints/Grid/BP_Grid.Is Tile Walkable` (`self.Grid Ref`) (`self.Target Index`))
          (if (<= (`self.Get Minimal Cost` (`self.Start Index`) (`self.Target Index`) (`self.Use Diagonals`)) (`self.Path Length`))
            (if (`KismetArrayLibrary.Array_Contains` (`self.Valid Types`) _tiletype)
              (if (not (`KismetSystemLibrary.IsValid` _unitontile))
                (return true)
                (else
                  (return false)))
              (else
                (return false)))
            (else
              (return false)))
          (else
            (return false)))
        (else
          (return true)))
      (else
        (return false)))
    (else
      (return false))))

(fn `Pull the Cheapest`
  (returns (`Cheapest Tile` :type "/Game/Blueprints/Grid/F_PathfindingData Structure"))
  (locals (`Tile Index` :type "IntPoint Structure"))
  (set `local.Tile Index` (`|GetArrayItem` (`self.Discovered Tiles`)))
  (`KismetArrayLibrary.Array_Remove` (`self.Discovered Tile Sorting Cost`))
  (`KismetArrayLibrary.Array_Remove` (`self.Discovered Tiles`))
  (`KismetArrayLibrary.Array_Add` (`self.Analysed Tiles`) (`local.Tile Index`))
  (return (`BlueprintMapLibrary.Map_Find` (`self.Pathfinding Data`) (`local.Tile Index`))))

(fn `Set Priority for Diagonals`
  (params (`Input Data` :type "/Game/Blueprints/Grid/F_PathfindingData Structure (by ref)"))
  (returns (Cost :type Integer))
  (bind (_index _previousindex _costtoentertile _costfromthestart _minimalcosttotarget) (break `/Game/Blueprints/Grid/F_PathfindingData` `Input Data`))
  (return (+ (`KismetMathLibrary.Conv_BoolToInt` (`self.Is Diagonal` _index _previousindex)) (* (+ _costfromthestart _minimalcosttotarget) 2))))

(fn `UserConstructionScript`)