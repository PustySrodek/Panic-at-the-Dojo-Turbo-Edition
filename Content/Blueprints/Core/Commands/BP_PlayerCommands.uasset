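; BP_PlayerCommands is the player's input controller for a grid-based combat game, tracking hovered and selected tiles and characters under the cursor.
; Left and right clicks delegate to swappable command actors spawned by SetSelectedCommand, which run on press and re-run while held as the hovered tile changes.
; Combat system and grid events drive selection, swap Move or CastAction commands, and create the combat menu and end screen.
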(event `self.ReceiveBeginPlay`
  (bind _combat_system (`self.Combat System`))
  (bind _grid (`self.Grid`))
  (bind _returnvalue (`GameplayStatics.GetActorOfClass` "/Game/Blueprints/Grid/BP_Grid.BP_Grid_C"))
  (set `self.Grid` _returnvalue)
  (bind _returnvalue_2 (`GameplayStatics.GetActorOfClass` "/Game/Blueprints/Core/Combat/BP_CombatSystem.BP_CombatSystem_C"))
  (bind _output_get (set `self.Combat System` _returnvalue_2))
  (add `/Game/Blueprints/Core/Combat/BP_CombatSystem.On Character Grid Index Change` _output_get (`|CreateDelegate` :!event `Character Grid Index Change`))
  (add `/Game/Blueprints/Grid/BP_Grid.OnGridGenerated` _grid (`|CreateDelegate` :!event `Update On Grid Generated`))
  (add `/Game/Blueprints/Grid/BP_Grid.OnTileDataUpdated` _grid (`|CreateDelegate` :!event `Update on Tile Updated`))
  (add `/Game/Blueprints/Core/Combat/BP_CombatSystem.On Combat Ended` _combat_system (`|CreateDelegate` :!event `Set on Combat End`))
  (add `/Game/Blueprints/Core/Combat/BP_CombatSystem.On Combat Start` _combat_system (`|CreateDelegate` :!event `Set on Combat Start`))
  (add `/Game/Blueprints/Core/Combat/BP_CombatSystem.On Character Turn Started` _combat_system (`|CreateDelegate` :!event `Character Turn Started`))
  (add `/Game/Blueprints/Core/Combat/BP_CombatSystem.On Character Turn Ended` _combat_system (`|CreateDelegate` :!event `Character Turn Ended`))
  (add `/Game/Blueprints/Core/Combat/BP_CombatSystem.On Finishing Combat` _combat_system (`|CreateDelegate` :!event `Set on Combat Finishing`))
  (`self.EnableInput` (`GameplayStatics.GetPlayerController` 0))
  (`self.Set Selected Command` null))

(event `self.ReceiveTick`
  (params (DeltaSeconds :type "Float (single-precision)"))
  (`self.Update Tile Under Cursor`))

(event `EnhancedInput|/Game/Inputs/IA_ActionExecute`
  (params (ActionValue :type Boolean) (ElapsedSeconds :type "Float (double-precision)") (TriggeredSeconds :type "Float (double-precision)") (InputAction :type "InputAction Object Reference" :default "/Game/Inputs/IA_ActionExecute.IA_ActionExecute"))
  (:`Triggered`
    (if ActionValue
      (`self.Update Tile Under Cursor`)
      (set `self.Left Click Down` true)
      (`/Engine/EditorBlueprintResources/StandardMacros.IsValid` (`self.Selected Left Click`)
        (:`Is Valid`
          (`/Game/Blueprints/Core/Commands/BP_Command.Execute Action` (`self.Selected Left Click`) (`self.Hovered Tile`) :!label _label)))
      (else
        (set `self.Left Click Down` false)))))

(event `On Hovered Tile`
  (bind _selected_right_click (`self.Selected Right Click`))
  (bind _selected_left_click (`self.Selected Left Click`))
  (`|ExecutionSequence`
    (:`then_0`
      (`/Engine/EditorBlueprintResources/StandardMacros.IsValid` _selected_left_click
        (:`Is Valid`
          (`/Game/Blueprints/Core/Commands/BP_Command.Execute Hovered Action` _selected_left_click (`self.Hovered Tile`))
          (if (`self.Left Click Down`)
            (goto _label)))))
    (:`then_1`
      (`/Engine/EditorBlueprintResources/StandardMacros.IsValid` _selected_right_click
        (:`Is Valid`
          (`/Game/Blueprints/Core/Commands/BP_Command.Execute Hovered Action` _selected_right_click (`self.Hovered Tile`))
          (if (`self.Right Click Down`)
            (`/Game/Blueprints/Core/Commands/BP_Command.Execute Action` (`self.Selected Right Click`) (`self.Hovered Tile`) :!label _label_2)))))))

(event `EnhancedInput|/Game/Inputs/IA_Action2Execute`
  (params (ActionValue :type Boolean) (ElapsedSeconds :type "Float (double-precision)") (TriggeredSeconds :type "Float (double-precision)") (InputAction :type "InputAction Object Reference" :default "/Game/Inputs/IA_Action2Execute.IA_Action2Execute"))
  (:`Triggered`
    (if ActionValue
      (`self.Update Tile Under Cursor`)
      (set `self.Right Click Down` true)
      (`/Engine/EditorBlueprintResources/StandardMacros.IsValid` (`self.Selected Right Click`)
        (:`Is Valid`
          (goto _label_2)))
      (else
        (set `self.Right Click Down` false)))))

(fn `Can Hover Empty Space`
  (returns (`Return Value` :type Boolean))
  (return (`KismetArrayLibrary.Array_Contains` (`|MakeArray` (`GameplayStatics.GetObjectClass` (`self.Selected Left Click`)) (`GameplayStatics.GetObjectClass` (`self.Selected Right Click`))) "/Game/Blueprints/Core/Commands/Grid/Command_AddTile.Command_AddTile_C")))

(fn `Character Grid Index Change`
  (params (Character :type "/Game/Blueprints/Characters/BP_Character Object Reference"))
  (if (== Character (`self.Selected Character`))
    (`self.Set Selected Tile and Character` (`/Game/Blueprints/Characters/BP_Character.Grid Index` (`local.Character`)))))

(fn `Character Turn Ended`
  (params (character :type "/Game/Blueprints/Characters/BP_Character Object Reference"))
  (`self.Set Selected Tile and Character` (make `IntPoint` -999 -999))
  (`self.Set Selected Command` null)
  (`/Game/Blueprints/HUD/Debug_Menu/Buttons/ButtonList_Actions.Link Action Bar to Character` (`/Game/Blueprints/HUD/Combat_Menu/WBP_CombatMenu.ButtonList_Actions` (`self.Combat Menu`)) null)
  (`/Game/Blueprints/HUD/Debug_Menu/Buttons/ButtonList_ActionDice.Link Dice Bar to Character` (`/Game/Blueprints/HUD/Combat_Menu/WBP_CombatMenu.ButtonList_ActionDice` (`self.Combat Menu`)) null))

(fn `Character Turn Started`
  (params (character :type "/Game/Blueprints/Characters/BP_Character Object Reference"))
  (`self.Set Selected Tile and Character` (`/Game/Blueprints/Characters/BP_Character.Grid Index` character))
  (`self.Set Selected Command` "/Game/Blueprints/Core/Commands/Combat/CCommand_Move.CCommand_Move_C")
  (`/Game/Blueprints/HUD/Debug_Menu/Buttons/ButtonList_Actions.Link Action Bar to Character` (`/Game/Blueprints/HUD/Combat_Menu/WBP_CombatMenu.ButtonList_Actions` (`self.Combat Menu`)) (`local.character`))
  (`/Game/Blueprints/HUD/Debug_Menu/Buttons/ButtonList_ActionDice.Link Dice Bar to Character` (`/Game/Blueprints/HUD/Combat_Menu/WBP_CombatMenu.ButtonList_ActionDice` (`self.Combat Menu`)) (`local.character`))
  (`/Game/Blueprints/HUD/Combat_Menu/WBP_TokenTracker.Link Token Numbers` (`/Game/Blueprints/HUD/Combat_Menu/WBP_CombatMenu.WBP_TokenTracker` (`self.Combat Menu`)) (`local.character`)))

(fn `Get Character Under Cursor`
  (params (PlayerIndex :type Integer))
  (returns (Character :type "/Game/Blueprints/Characters/BP_Character Object Reference"))
  (bind (_hitresult _returnvalue) (`PlayerController.GetHitResultUnderCursorByChannel` (`GameplayStatics.GetPlayerController` PlayerIndex) "TraceTypeQuery5" false))
  (if _returnvalue
    (return (cast `/Game/Blueprints/Characters/BP_Character` (`.HitActor` (`GameplayStatics.BreakHitResult` _hitresult)) :!pure true))
    (else
      (bind _index (`/Game/Blueprints/Grid/BP_Grid.Get Tile Under Cursor` (`self.Grid`) (`local.PlayerIndex`) true (`self.Can Hover Empty Space`)))
      (return (`.UnitonTile_19_090F5A1342BB3758B627C38D844712AB` (break `/Game/Blueprints/Grid/F_TileData` (`BlueprintMapLibrary.Map_Find` (`/Game/Blueprints/Grid/BP_Grid.Grid Tiles Data` (`self.Grid`)) _index)))))))

(fn `Set on Combat End`
  (`Widget.RemoveFromParent` (`self.Combat End Screen`))
  (set `self.Combat End Screen` null))

(fn `Set on Combat Finishing`
  (params (`Wining Team Index` :type Integer))
  (`self.Set Selected Command` null)
  (`self.Set Selected Tile and Character` (make `IntPoint` -999 -999))
  (`Widget.RemoveFromParent` (`self.Combat Menu`))
  (set `self.Combat Menu` null)
  (bind _returnvalue (`|CreateWidget` "/Game/Blueprints/HUD/Combat_Menu/WBP_CombatEndScreen.WBP_CombatEndScreen_C" null (`local.Wining Team Index`) self))
  (bind _output_get (set `self.Combat End Screen` _returnvalue))
  (`UserWidget.AddToPlayerScreen` _output_get 0))

(fn `Set on Combat Start`
  (`self.Set Selected Command` null)
  (`self.Set Selected Tile and Character` (make `IntPoint` -999 -999))
  (bind _returnvalue (`|CreateWidget` "/Game/Blueprints/HUD/Combat_Menu/WBP_CombatMenu.WBP_CombatMenu_C" null self))
  (bind _output_get (set `self.Combat Menu` _returnvalue))
  (`UserWidget.AddToPlayerScreen` _output_get 0)
  (add `/Game/Blueprints/HUD/Debug_Menu/Buttons/ButtonList_Actions.OnSelectedActionButtonChange` (`/Game/Blueprints/HUD/Combat_Menu/WBP_CombatMenu.ButtonList_Actions` (`self.Combat Menu`)) (`|CreateDelegate` :!event `Set Selected Action`))
  (add `/Game/Blueprints/HUD/Debug_Menu/Buttons/ButtonList_ActionDice.OnSelectedDieButtonChange` (`/Game/Blueprints/HUD/Combat_Menu/WBP_CombatMenu.ButtonList_ActionDice` (`self.Combat Menu`)) (`|CreateDelegate` :!event `Set Selected Die`)))

(fn `Set Selected Action`
  (params (Button :type "/Game/Blueprints/HUD/Debug_Menu/Buttons/Button_Action Object Reference"))
  (`/Engine/EditorBlueprintResources/StandardMacros.IsValid` Button
    (:`Is Valid`
      (`self.Set Selected Command` "/Game/Blueprints/Core/Commands/Combat/CCommand_CastAction.CCommand_CastAction_C")
      (bind _asccommand_cast_action (cast `/Game/Blueprints/Core/Commands/Combat/CCommand_CastAction` (`self.Selected Left Click`)))
      (`/Game/Blueprints/Core/Commands/Combat/CCommand_CastAction.Set Action` _asccommand_cast_action (`/Game/Blueprints/HUD/Debug_Menu/Buttons/Button_Action.Action` (`local.Button`))))
    (:`Is Not Valid`
      (if (!= (`GameplayStatics.GetObjectClass` (`self.Selected Left Click`)) "/Game/Blueprints/Core/Commands/Combat/CCommand_Move.CCommand_Move_C")
        (`self.Set Selected Command` "/Game/Blueprints/Core/Commands/Combat/CCommand_Move.CCommand_Move_C")))))

(fn `Set Selected Command`
  (params (`Left Action` :type "/Game/Blueprints/Core/Commands/BP_Command Class Reference") (`Right Action` :type "/Game/Blueprints/Core/Commands/BP_Command Class Reference"))
  (bind _selected_right_click (`self.Selected Right Click`))
  (bind _selected_left_click (`self.Selected Left Click`))
  (bind _left_action (`local.Left Action`))
  (bind _right_action (`local.Right Action`))
  (`|ExecutionSequence`
    (:`then_0`
      (`/Engine/EditorBlueprintResources/StandardMacros.IsValid` _selected_left_click
        (:`Is Valid`
          (`self.K2_DestroyActor` _selected_left_click)
          (set `self.Selected Left Click` null))
        (:`Is Not Valid`
          _))
      (if (`KismetSystemLibrary.IsValidClass` _left_action)
        (bind _returnvalue (`|SpawnActorFromClass` _left_action (`KismetMathLibrary.MakeTransform` (0.0 0.0 0.0)) "AlwaysSpawn" "MultiplyWithRoot" null self null))
        (set `self.Selected Left Click` _returnvalue)))
    (:`then_1`
      (`/Engine/EditorBlueprintResources/StandardMacros.IsValid` _selected_right_click
        (:`Is Valid`
          (`self.K2_DestroyActor` _selected_right_click)
          (set `self.Selected Right Click` null))
        (:`Is Not Valid`
          _))
      (if (`KismetSystemLibrary.IsValidClass` _right_action)
        (bind _returnvalue_2 (`|SpawnActorFromClass` _right_action (`KismetMathLibrary.MakeTransform` (0.0 0.0 0.0)) "AlwaysSpawn" "MultiplyWithRoot" null self null))
        (set `self.Selected Right Click` _returnvalue_2)))
    (:`then_2`
      (`self.On Selected Command Change` (`self.Selected Left Click`) (`self.Selected Right Click`)))))

(fn `Set Selected Die`
  (params (Button :type "/Game/Blueprints/HUD/Debug_Menu/Buttons/Button_ActionDie Object Reference"))
  (`/Engine/EditorBlueprintResources/StandardMacros.IsValid` Button
    (:`Is Valid`
      (`/Game/Blueprints/Characters/BP_Character.Set Selected Number and Index` (`/Game/Blueprints/Core/Combat/BP_CombatSystem.Current Acting Character` (`self.Combat System`)) (`/Game/Blueprints/HUD/Debug_Menu/Buttons/Button_ActionDie.Action Die` Button) (`/Game/Blueprints/HUD/Debug_Menu/Buttons/Button_ActionDie.Die Index` Button))
      (if (!= (`GameplayStatics.GetObjectClass` (`self.Selected Left Click`)) "/Game/Blueprints/Core/Commands/Combat/CCommand_Move.CCommand_Move_C")
        (`self.Set Selected Command` "/Game/Blueprints/Core/Commands/Combat/CCommand_Move.CCommand_Move_C")))))

(fn `Set Selected Tile and Character`
  (params (Index :type "IntPoint Structure") (Force :type Boolean))
  (locals (`New Character` :type "/Game/Blueprints/Characters/BP_Character Object Reference"))
  (bind _selected_character (`self.Selected Character`))
  (`|ExecutionSequence`
    (:`then_0`
      (if (or (!= (`local.Index`) (`self.Selected Tile`)) (`local.Force`))
        (`/Game/Blueprints/Grid/BP_Grid.Remove State from Tile` (`self.Grid`) (`self.Selected Tile`) "NewEnumerator2")
        (set `self.Selected Tile` (`local.Index`))
        (`/Game/Blueprints/Grid/BP_Grid.Add State to Tile` (`self.Grid`) (`self.Selected Tile`) "NewEnumerator2")
        (else
          (`/Game/Blueprints/Grid/BP_Grid.Remove State from Tile` (`self.Grid`) (`self.Selected Tile`) "NewEnumerator2")
          (set `self.Selected Tile` (make `IntPoint` -999 -999))))
      (`/Engine/EditorBlueprintResources/StandardMacros.IsValid` (`.UnitonTile_19_090F5A1342BB3758B627C38D844712AB` (break `/Game/Blueprints/Grid/F_TileData` (`BlueprintMapLibrary.Map_Find` (`/Game/Blueprints/Grid/BP_Grid.Grid Tiles Data` (`self.Grid`)) (`self.Selected Tile`))))
        (:`Is Not Valid`
          (set `self.Selected Character` null)
          (`self.On Selected Tile Change` (`self.Selected Tile`)))))
    (:`then_1`
      (bind _output_get (set `local.New Character` (`.UnitonTile_19_090F5A1342BB3758B627C38D844712AB` (break `/Game/Blueprints/Grid/F_TileData` (`BlueprintMapLibrary.Map_Find` (`/Game/Blueprints/Grid/BP_Grid.Grid Tiles Data` (`self.Grid`)) (`self.Selected Tile`))))))
      (if (!= _output_get (`self.Selected Character`))
        (`|ExecutionSequence`
          (:`then_0`
            (`/Engine/EditorBlueprintResources/StandardMacros.IsValid` _selected_character
              (:`Is Valid`
                (`/Game/Blueprints/Characters/BP_Character.Set is Selected` _selected_character false))))
          (:`then_1`
            (bind _output_get_2 (set `self.Selected Character` (`local.New Character`)))
            (`/Engine/EditorBlueprintResources/StandardMacros.IsValid` _output_get_2
              (:`Is Valid`
                (`/Game/Blueprints/Characters/BP_Character.Set is Selected` _output_get_2 true)
                (`self.On Selected Tile Change` (`self.Selected Tile`))))))))))

(fn `Update On Grid Generated`
  (if (not (`/Game/Blueprints/Core/Combat/BP_CombatSystem.Is In Combat` (`self.Combat System`)))
    (if (`/Game/Blueprints/Grid/BP_Grid.Is Index Valid` (`self.Grid`) (`self.Hovered Tile`))
      (`self.Set Selected Tile and Character` (`self.Hovered Tile`) true)
      (else
        (`self.Set Selected Tile and Character` (make `IntPoint` -999 -999))))))

(fn `Update on Tile Updated`
  (params (Index :type "IntPoint Structure"))
  (if (`KismetMathLibrary.Equal_IntPointIntPoint` Index (`self.Hovered Tile`))
    (`self.Update On Grid Generated`)))

(fn `Update Tile Under Cursor`
  (locals (`New Index` :type "IntPoint Structure"))
  (bind _hovered_character (`self.Hovered Character`))
  (`|ExecutionSequence`
    (:`then_0`
      (bind _character (`self.Get Character Under Cursor` 0))
      (if (!= _character (`self.Hovered Character`))
        (`/Engine/EditorBlueprintResources/StandardMacros.IsValid` _hovered_character
          (:`Is Valid`
            (`/Game/Blueprints/Characters/BP_Character.Set Is Hovered` _hovered_character false))
          (:`Is Not Valid`
            _))
        (bind _output_get (set `self.Hovered Character` _character))
        (`/Engine/EditorBlueprintResources/StandardMacros.IsValid` _output_get
          (:`Is Valid`
            (`/Game/Blueprints/Characters/BP_Character.Set Is Hovered` _output_get true)))))
    (:`then_1`
      (`/Engine/EditorBlueprintResources/StandardMacros.IsValid` (`self.Hovered Character`)
        (:`Is Valid`
          (set `local.New Index` (`/Game/Blueprints/Characters/BP_Character.Grid Index` (`self.Hovered Character`))))
        (:`Is Not Valid`
          (bind _index (`/Game/Blueprints/Grid/BP_Grid.Get Tile Under Cursor` (`self.Grid`) 0 true (`self.Can Hover Empty Space`)))
          (set `local.New Index` _index)))
      (if (!= (`local.New Index`) (`self.Hovered Tile`))
        (`/Game/Blueprints/Grid/BP_Grid.Remove State from Tile` (`self.Grid`) (`self.Hovered Tile`) "NewEnumerator1")
        (set `self.Hovered Tile` (`local.New Index`))
        (`/Game/Blueprints/Grid/BP_Grid.Add State to Tile` (`self.Grid`) (`self.Hovered Tile`) "NewEnumerator1")
        (`self.On Hovered Tile`)))))

(fn `UserConstructionScript`)