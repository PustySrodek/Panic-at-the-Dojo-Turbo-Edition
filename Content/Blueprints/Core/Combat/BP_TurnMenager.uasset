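; Turn manager for grid combat that tracks rounds and steps characters through stance, Heroic Spirit, action dice, movement, action/reaction and end-turn phases.
; UpdateTurnPhase increments the phase enum and broadcasts it, while dispatchers announce movement and action phases.
; AbilitiesHandler rolls dice, which Heroic Spirit can transfer to an ally.
; Turn end clears dice pools, reduces tokens, applies token-based damage and has CombatSystem change the active character.
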(event `self.ReceiveBeginPlay`
  (bind _returnvalue (`GameplayStatics.GetActorOfClass` "/Game/Blueprints/Core/Combat/BP_AbilitiesHandler.BP_AbilitiesHandler_C"))
  (set `self.Abilities Handler` _returnvalue))

(event `Initilize all player stance select`
  (for _array_element (`/Game/Blueprints/Core/Combat/BP_CombatSystem.Characters on Grid` (`self.Combat System`))
    (add `/Game/Blueprints/Character/BP_Character.On Character Stance Changed` _array_element (`|CreateDelegate` :!event `Check Player Stances`))))

(fn `Action and Reaction Phase`
  (`self.On Action Phase Activated`))

(fn `Action Dice Phase`
  (set `self.Turn Phase` "NewEnumerator3")
  (`/Game/Blueprints/Core/Combat/BP_AbilitiesHandler.Roll Dice For Character` (`self.Abilities Handler`) (`/Game/Blueprints/Core/Combat/BP_CombatSystem.Active Character` (`self.Combat System`)))
  (if (`KismetSystemLibrary.IsValid` (`self.Heroic Spirit Ally`))
    (for _array_element (`.ActionPool_5_B5573866494C04EA2C02C882EFD84F22` (break `/Game/Blueprints/Character/F_CharacterData_Stance` (`/Game/Blueprints/Character/BP_Character.Active Stance` (`self.Heroic Spirit Giver`))))
      (`/Game/Blueprints/Character/BP_Character.Modify Character Action Pool` (`self.Heroic Spirit Ally`) true 0 _array_element))
    (`/Game/Blueprints/Character/BP_Character.Modify Character Action Pool` (`self.Heroic Spirit Giver`) false -1 0)
    (`self.Update Turn Phase`)
    (`self.Movement Phase`)
    (else
      (`self.Update Turn Phase`)
      (`self.Movement Phase`))))

(fn `Activate After Movement Phase`
  (switch `/Game/Blueprints/Core/Combat/Utility/Enum_TurnPhase` (`self.Turn Phase`)
    (:`NewEnumerator5`
      (`self.Action and Reaction Phase`)
      (`KismetSystemLibrary.PrintString` "Action Phase"))
    (:`NewEnumerator7`
      (`self.Turn Ends` (`/Game/Blueprints/Core/Combat/BP_CombatSystem.Active Character` (`self.Combat System`))))))

(fn `Activate Start of Turn Abilities`
  (params (Character :type "/Game/Blueprints/Character/BP_Character Object Reference"))
  (bind _character (`local.Character`))
  (if (or (`/Game/Blueprints/Character/BP_Character.Check is Dead` _character) (`/Game/Blueprints/Character/BP_Character.Removed from play` _character))
    (`self.Update Turn Phase`)
    (`self.Initilize Heroic Spirit` (`local.Character`))
    (else
      (set `self.Turn Phase` "NewEnumerator2")
      (`self.Update Turn Phase`)
      (`self.Action Dice Phase`))))

(fn `Check Player Stances`
  (params (Character :type "/Game/Blueprints/Character/BP_Character Object Reference"))
  (bind _combat_system (`self.Combat System`))
  (bind _output_get (set `self.Stances Selected` (+ (`self.Stances Selected`) 1)))
  (if (== _output_get (`KismetArrayLibrary.Array_Length` (`/Game/Blueprints/Core/Combat/BP_CombatSystem.Characters on Grid` (`self.Combat System`))))
    (for _array_element (`/Game/Blueprints/Core/Combat/BP_CombatSystem.Characters on Grid` (`self.Combat System`))
      (clear `/Game/Blueprints/Character/BP_Character.On Character Stance Changed` _array_element)
      (add `/Game/Blueprints/Character/BP_Character.On Character Stance Changed` _array_element (`|CreateDelegate` :!event `Activate Start of Turn Abilities`)))
    (bind _new_active_character (`/Game/Blueprints/Core/Combat/BP_CombatSystem.Set Active Character By Ref` _combat_system (`|GetArrayItem` (`/Game/Blueprints/Core/Combat/BP_CombatSystem.Characters on Grid` _combat_system))))
    (`/Game/Blueprints/Core/Combat/BP_CombatSystem.Set Current Acting Character By Ref` (`self.Combat System`) _new_active_character)))

(fn `Initilize Heroic Spirit`
  (params (Character :type "/Game/Blueprints/Character/BP_Character Object Reference"))
  (bind _returnvalue (`|CreateWidget` "/Game/Blueprints/HUD/Combat_Menu/HeroicSpirit/WBP_HeroicSpirit.WBP_HeroicSpirit_C" null self Character))
  (`UserWidget.AddToPlayerScreen` _returnvalue 0))

(fn `Movement Phase`
  (locals (`Valid for Movement` :type "Array of /Game/Blueprints/Character/BP_Character Object Reference") (`Loop Character` :type "/Game/Blueprints/Character/BP_Character Object Reference"))
  (for _array_element (`/Game/Blueprints/Core/Combat/BP_CombatSystem.Characters on Grid` (`self.Combat System`))
    (bind _output_get (set `local.Loop Character` _array_element))
    (if (> (`BlueprintMapLibrary.Map_Find` (`.Tokens_73_F3A6EA8D45314AD8E266579E853C1E32` (break `/Game/Blueprints/Character/F_CharacterData_Stats` (`.Stats_8_5DCC378E48218015EE4248AF0BBAB223` (break `/Game/Blueprints/Character/F_CharacterData` (`/Game/Blueprints/Character/BP_Character.Character Data` _output_get))))) "NewEnumerator0") 0)
      (`KismetArrayLibrary.Array_Add` (`self.Valid For Movement_0`) (`local.Loop Character`))))
  (if (`KismetArrayLibrary.Array_IsEmpty` (`local.Valid for Movement`))
    (`self.Update Turn Phase`)
    (`self.Activate After Movement Phase`)
    (else
      (`self.On Movement Activated`))))

(fn `Set on Combat Start`
  (set `self.Current Round` 0)
  (set `self.Stances Selected` 0)
  (set `self.Turn Phase` "NewEnumerator8"))

(fn `Start of Round`
  (params (Character :type "/Game/Blueprints/Character/BP_Character Object Reference"))
  (if (> (`self.Current Round`) 1)
    (`self.Update Turn Phase`)
    (`/Game/Blueprints/Character/BP_Character.Select Stance` (`local.Character`))
    (else
      (set `self.Turn Phase` "NewEnumerator0")
      (`self.Update Turn Phase`)
      (`self.Activate Start of Turn Abilities` (`local.Character`)))))

(fn `Turn Ends`
  (params (character :type "/Game/Blueprints/Character/BP_Character Object Reference"))
  (bind _combat_system (`self.Combat System`))
  (bind _combat_system_2 (`self.Combat System`))
  (bind _returnvalue (- 0 (`KismetMathLibrary.Round` (/ (`KismetMathLibrary.Conv_IntToDouble` (`BlueprintMapLibrary.Map_Find` (`.Tokens_73_F3A6EA8D45314AD8E266579E853C1E32` (break `/Game/Blueprints/Character/F_CharacterData_Stats` (`.Stats_8_5DCC378E48218015EE4248AF0BBAB223` (break `/Game/Blueprints/Character/F_CharacterData` (`/Game/Blueprints/Character/BP_Character.Character Data` (`local.character`)))))) "NewEnumerator6")) 2.0))))
  (for _array_element (`/Game/Blueprints/Core/Combat/BP_CombatSystem.Characters on Grid` (`self.Combat System`))
    (`/Game/Blueprints/Character/BP_Character.Modify Current Tokens` _array_element -3 "NewEnumerator0")
    (for (_ _array_index) (`.ActionPool_5_B5573866494C04EA2C02C882EFD84F22` (break `/Game/Blueprints/Character/F_CharacterData_Stance` (`/Game/Blueprints/Character/BP_Character.Active Stance` _array_element)))
      (`/Game/Blueprints/Character/BP_Character.Modify Character Action Pool` _array_element false _array_index 0)))
  (if (`/Game/Blueprints/Character/BP_Character.Moved This turn` (`local.character`))
    (set `/Game/Blueprints/Character/BP_Character.Moved This turn` false (`local.character`)))
  (`/Game/Blueprints/Core/Combat/BP_CombatSystem.Process Hits` :`self` (`self.Combat System`) :`Impact Data` (make `/Game/Blueprints/Core/Combat/Actions/Utility/F_ActionImpact` _returnvalue _returnvalue) :`character Ovveride` (`local.character`))
  (`/Game/Blueprints/Character/BP_Character.Modify Current Tokens` (`local.character`) _returnvalue "NewEnumerator6")
  (`/Engine/EditorBlueprintResources/StandardMacros.IsValid` (`self.Heroic Spirit Giver`)
    (:`Is Valid`
      (set `self.Heroic Spirit Ally` null)
      (bind _output_get (set `/Game/Blueprints/Core/Combat/BP_CombatSystem.Active Character` (`self.Heroic Spirit Giver`) _combat_system))
      (set `/Game/Blueprints/Core/Combat/BP_CombatSystem.Current Acting Character` _output_get _combat_system))
    (:`Is Not Valid`
      _))
  (`/Game/Blueprints/Core/Combat/BP_CombatSystem.Change Active Character` _combat_system_2)
  (`/Game/Blueprints/Core/Combat/BP_CombatSystem.Change Current Acting Character` _combat_system_2))

(fn `Turn Starts`
  (params (Character :type "/Game/Blueprints/Character/BP_Character Object Reference"))
  (set `self.Heroic Spirit Giver` null)
  (set `self.Heroic Spirit Ally` null)
  (if (== (`KismetArrayLibrary.Array_Find` (`/Game/Blueprints/Core/Combat/BP_CombatSystem.Characters on Grid` (`self.Combat System`)) (`local.Character`)) 0)
    (set `self.Current Round` (+ (`self.Current Round`) 1))
    (`self.Start of Round` (`local.Character`))
    (return)
    (else
      (`self.Update Turn Phase`)
      (`/Game/Blueprints/Character/BP_Character.Select Stance` (`local.Character`)))))

(fn `Update Turn Phase`
  (bind _output_get (set `self.Turn Phase` (cast `/Game/Blueprints/Core/Combat/Utility/Enum_TurnPhase` (`KismetMathLibrary.Conv_IntToByte` (+ (`KismetMathLibrary.Conv_ByteToInt` (`self.Turn Phase`)) 1)))))
  (`self.On Turn Phase Changed` _output_get))

(fn `UserConstructionScript`)