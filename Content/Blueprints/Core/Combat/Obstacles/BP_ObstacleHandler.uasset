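; Combat obstacle handler that places, moves, removes and damages obstacles such as walls, rubble, traps, pits, fog and copies on the grid.
; Index changes rewrite each tile's type-keyed obstacle map, resolve stacking conflicts by destroying obstacles, and fire add/remove notifications.
; A tile-update handler re-snaps obstacles or destroys those on missing tiles.
; Damage instantly removes walls, rubble or copies past type-specific thresholds, without tracking health.
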(event `self.ReceiveBeginPlay`
  (`KismetSystemLibrary.Delay` 0.5)
  (add `/Game/Blueprints/Grid/BP_Grid.OnTileDataUpdated` (`/Game/Blueprints/Core/Combat/BP_CombatSystem.Grid Ref` (`self.Combat System`)) (`|CreateDelegate` :!event `Set Obstacle on Tile Data Updated`)))

(fn `Add Obstacle To Grid`
  (params (Index :type "IntPoint Structure") (Obstacle :type "/Game/Blueprints/Core/Combat/Obstacles/ObstacleClasses/BP_Obstacle Object Reference"))
  (`self.Set Obstacle Index` Index Obstacle false true)
  (`/Engine/EditorBlueprintResources/StandardMacros.IsValid` Obstacle
    (:`Is Valid`
      (`KismetArrayLibrary.Array_Add` (`self.Obstacles on grid`) (`local.Obstacle`))
      (`/Game/Blueprints/Core/Combat/Obstacles/ObstacleClasses/BP_Obstacle.Set Obstacle Handler` (`local.Obstacle`) self))))

(fn `Addi Obstacle to Tile`
  (params (`Obstacle Type` :type "/Game/Blueprints/Core/Combat/Obstacles/Utility/Enum_Obstacles Enum" :default "NewEnumerator6") (`Next Tile` :type "/Game/Blueprints/Grid/F_TileData Structure") (Obstacle :type "/Game/Blueprints/Core/Combat/Obstacles/ObstacleClasses/BP_Obstacle Object Reference"))
  (bind (_value _returnvalue) (`BlueprintMapLibrary.Map_Find` (`.Obstacles_25_D60D9EA04845E620E0A0308708D4894E` (break `/Game/Blueprints/Grid/F_TileData` (`local.Next Tile`))) "NewEnumerator11"))
  (bind (_value_2 _returnvalue_2) (`BlueprintMapLibrary.Map_Find` (`.Obstacles_25_D60D9EA04845E620E0A0308708D4894E` (break `/Game/Blueprints/Grid/F_TileData` (`local.Next Tile`))) "NewEnumerator12"))
  (switch `/Game/Blueprints/Core/Combat/Obstacles/Utility/Enum_Obstacles` `Obstacle Type`
    (:`NewEnumerator7`
      (if _returnvalue :!label _label
        (`self.Remove Obstacle From Grid` _value true)
        (`self.Remove Obstacle From Grid` (`local.Obstacle`) true)
        (elif _returnvalue_2
          (`self.Remove Obstacle From Grid` _value_2 true)
          (`self.Remove Obstacle From Grid` (`local.Obstacle`) true)
          (else
            (`BlueprintMapLibrary.Map_Add` (`.Obstacles_25_D60D9EA04845E620E0A0308708D4894E` (break `/Game/Blueprints/Grid/F_TileData` (`local.Next Tile`))) (`local.Obstacle Type`) (`local.Obstacle`) :!label _label_2)
            (`BlueprintMapLibrary.Map_Add` (`/Game/Blueprints/Grid/BP_Grid.Grid Tiles Data` (`/Game/Blueprints/Core/Combat/BP_CombatSystem.Grid Ref` (`self.Combat System`))) (`/Game/Blueprints/Core/Combat/Obstacles/ObstacleClasses/BP_Obstacle.Obstacle Index` (`local.Obstacle`)) (`local.Next Tile`))
            (`self.On Obstacle Added to Index` (`local.Obstacle`))))))
    (:`NewEnumerator8`
      (goto _label))
    (:`NewEnumerator9`
      (if (not (`BlueprintMapLibrary.Map_Contains` (`.Obstacles_25_D60D9EA04845E620E0A0308708D4894E` (break `/Game/Blueprints/Grid/F_TileData` (`local.Next Tile`))) "NewEnumerator9"))
        (goto _label_2)
        (else
          (`self.Remove Obstacle From Grid` (`local.Obstacle`) true))))
    (:`NewEnumerator10`
      (goto _label))
    (:`NewEnumerator11`
      (bind _values (`BlueprintMapLibrary.Map_Values` (`.Obstacles_25_D60D9EA04845E620E0A0308708D4894E` (break `/Game/Blueprints/Grid/F_TileData` (`local.Next Tile`))) :!label _label_3))
      (for _array_element _values
        (`self.Remove Obstacle From Grid` _array_element true))
      (goto _label_2))
    (:`NewEnumerator12`
      (goto _label_3))))

(fn `Damage Obstacle`
  (params (Obstacle :type "/Game/Blueprints/Core/Combat/Obstacles/ObstacleClasses/BP_Obstacle Object Reference") (damage :type Integer))
  (bind _obstacle_type (`/Game/Blueprints/Core/Combat/Obstacles/ObstacleClasses/BP_Obstacle.Obstacle Type` Obstacle))
  (if (or (and (or (`|EnumEquality` _obstacle_type "NewEnumerator11") (`|EnumEquality` _obstacle_type "NewEnumerator12")) (<= (`local.damage`) -2)) (and (`|EnumEquality` _obstacle_type "NewEnumerator10") (<= (`local.damage`) -1)))
    (`self.Remove Obstacle From Grid` (`local.Obstacle`) true)))

(fn `Remove Obstacle From Grid`
  (params (Obstacle :type "/Game/Blueprints/Core/Combat/Obstacles/ObstacleClasses/BP_Obstacle Object Reference") (`Destroy?` :type Boolean))
  (`self.Set Obstacle Index` (make `IntPoint` -999 -999) Obstacle false true)
  (if (`local.Destroy?`)
    (`self.K2_DestroyActor` (`local.Obstacle`))))

(fn `Set Obstacle Index`
  (params (Index :type "IntPoint Structure") (Obstacle :type "/Game/Blueprints/Core/Combat/Obstacles/ObstacleClasses/BP_Obstacle Object Reference") (Force :type Boolean) (`Snap Actor` :type Boolean))
  (locals (`Previous Tile` :type "/Game/Blueprints/Grid/F_TileData Structure") (`Next Tile` :type "/Game/Blueprints/Grid/F_TileData Structure") (`Obstacle Type` :type "/Game/Blueprints/Core/Combat/Obstacles/Utility/Enum_Obstacles Enum"))
  (bind _obstacle (`local.Obstacle`))
  (bind (_value _returnvalue) (`BlueprintMapLibrary.Map_Find` (`/Game/Blueprints/Grid/BP_Grid.Grid Tiles Data` (`/Game/Blueprints/Core/Combat/BP_CombatSystem.Grid Ref` (`self.Combat System`))) (`local.Index`)))
  (`/Engine/EditorBlueprintResources/StandardMacros.IsValid` Obstacle
    (:`Is Valid`
      (set `local.Obstacle Type` (`/Game/Blueprints/Core/Combat/Obstacles/ObstacleClasses/BP_Obstacle.Obstacle Type` Obstacle))
      (`|ExecutionSequence`
        (:`then_0`
          (if (or (!= (`/Game/Blueprints/Core/Combat/Obstacles/ObstacleClasses/BP_Obstacle.Obstacle Index` (`local.Obstacle`)) (`local.Index`)) (`local.Force`))
            (`|ExecutionSequence`
              (:`then_0`
                (bind _output_get (set `local.Previous Tile` (`BlueprintMapLibrary.Map_Find` (`/Game/Blueprints/Grid/BP_Grid.Grid Tiles Data` (`/Game/Blueprints/Core/Combat/BP_CombatSystem.Grid Ref` (`self.Combat System`))) (`/Game/Blueprints/Core/Combat/Obstacles/ObstacleClasses/BP_Obstacle.Obstacle Index` (`local.Obstacle`)))))
                (bind (_index _tiletype _tiletransform _tilestate _unitontile _obstacles) (break `/Game/Blueprints/Grid/F_TileData` _output_get))
                (if (`.ReturnValue` (`BlueprintMapLibrary.Map_Find` _obstacles (`local.Obstacle Type`)))
                  (`BlueprintMapLibrary.Map_Remove` _obstacles (`local.Obstacle Type`))
                  (`BlueprintMapLibrary.Map_Add` (`/Game/Blueprints/Grid/BP_Grid.Grid Tiles Data` (`/Game/Blueprints/Core/Combat/BP_CombatSystem.Grid Ref` (`self.Combat System`))) (`/Game/Blueprints/Core/Combat/Obstacles/ObstacleClasses/BP_Obstacle.Obstacle Index` (`local.Obstacle`)) (`local.Previous Tile`))))
              (:`then_1`
                (if (or (!= (`local.Index`) (make `IntPoint` -999 -999)) false)
                  (set `/Game/Blueprints/Core/Combat/Obstacles/ObstacleClasses/BP_Obstacle.Obstacle Index` (`local.Index`) (`local.Obstacle`))
                  (set `local.Next Tile` (`BlueprintMapLibrary.Map_Find` (`/Game/Blueprints/Grid/BP_Grid.Grid Tiles Data` (`/Game/Blueprints/Core/Combat/BP_CombatSystem.Grid Ref` (`self.Combat System`))) (`local.Index`)))
                  (`self.Addi Obstacle to Tile` (`local.Obstacle Type`) (`local.Next Tile`) (`local.Obstacle`))))
              (:`then_2`
                (`self.On Obstacle Removed From Index` (`local.Obstacle`))))))
        (:`then_1`
          (if (`local.Snap Actor`)
            (`/Engine/EditorBlueprintResources/StandardMacros.IsValid` _obstacle
              (:`Is Valid`
                (`self.K2_SetActorLocation` _obstacle (select `bool` _returnvalue :`false` (-999.0 -999.0 -999.0) :`true` (.location (`.TileTransform_9_C8B49F424080CB25DC8191A7EE85CF00` (break `/Game/Blueprints/Grid/F_TileData` _value)))) false true)))))))))

(fn `Set Obstacle on Tile Data Updated`
  (params (Index :type "IntPoint Structure"))
  (locals (`Tile Data` :type "/Game/Blueprints/Grid/F_TileData Structure"))
  (bind (_value _returnvalue) (`BlueprintMapLibrary.Map_Find` (`/Game/Blueprints/Grid/BP_Grid.Grid Tiles Data` (`/Game/Blueprints/Core/Combat/BP_CombatSystem.Grid Ref` (`self.Combat System`))) Index))
  (if _returnvalue
    (bind _output_get (set `local.Tile Data` _value))
    (bind _values (`BlueprintMapLibrary.Map_Values` (`.Obstacles_25_D60D9EA04845E620E0A0308708D4894E` (break `/Game/Blueprints/Grid/F_TileData` _output_get))))
    (for _array_element _values
      (`self.Set Obstacle Index` (`local.Index`) _array_element false true))
    (else
      (for _ (range 2)
        (for _array_element_2 (`self.Obstacles on grid`)
          (if (`KismetMathLibrary.Equal_IntPointIntPoint` (`/Game/Blueprints/Core/Combat/Obstacles/ObstacleClasses/BP_Obstacle.Obstacle Index` _array_element_2) (`local.Index`))
            (`self.Remove Obstacle From Grid` _array_element_2 true)))))))

(fn `UserConstructionScript`)