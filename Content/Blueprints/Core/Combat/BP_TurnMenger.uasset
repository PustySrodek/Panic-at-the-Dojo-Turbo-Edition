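; Turn manager for grid combat that gates combat start on stance selection and handles end-of-turn cleanup.
; It listens for stance changes, collects characters, then starts combat via CombatSystem once the count matches those on the grid.
; Turn end reduces one token type and updates action pools for all characters.
; The ending character's move flag resets, and half of another token becomes an HP change through ProcessHits and is removed.
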(event `Initilize all player stance select`
  (for _array_element (`/Game/Blueprints/Core/Combat/BP_CombatSystem.Characters on Grid` (`self.Combat System`))
    (add `/Game/Blueprints/Character/BP_Character.On Character Stance Changed` _array_element (`|CreateDelegate` :!event `Check Player Stances`))))

(fn `Check Player Stances`
  (params (Character :type "/Game/Blueprints/Character/BP_Character Object Reference"))
  (bind _returnvalue (`KismetArrayLibrary.Array_Add` (`self.Characters with Stances`) Character))
  (if (== (+ _returnvalue 1) (`KismetArrayLibrary.Array_Length` (`/Game/Blueprints/Core/Combat/BP_CombatSystem.Characters on Grid` (`self.Combat System`))))
    (`/Game/Blueprints/Core/Combat/BP_CombatSystem.Start Combat` (`self.Combat System`))
    (`self.On All Players Selected Stance`)))

(fn `Set on Combat Start`
  (`KismetArrayLibrary.Array_Clear` (`self.Characters with Stances`))
  (set `self.Current Round` 0))

(fn `Turn Ends`
  (params (character :type "/Game/Blueprints/Character/BP_Character Object Reference"))
  (bind _returnvalue (- 0 (`KismetMathLibrary.Round` (/ (`KismetMathLibrary.Conv_IntToDouble` (`BlueprintMapLibrary.Map_Find` (`.Tokens_73_F3A6EA8D45314AD8E266579E853C1E32` (break `/Game/Blueprints/Character/F_CharacterData_Stats` (`.Stats_8_5DCC378E48218015EE4248AF0BBAB223` (break `/Game/Blueprints/Character/F_CharacterData` (`/Game/Blueprints/Character/BP_Character.Character Data` (`local.character`)))))) "NewEnumerator6")) 2.0))))
  (for _array_element (`/Game/Blueprints/Core/Combat/BP_CombatSystem.Characters on Grid` (`self.Combat System`))
    (`/Game/Blueprints/Character/BP_Character.Modify Current Tokens` _array_element -3 "NewEnumerator0")
    (for (_ _array_index) (`.ActionPool_5_B5573866494C04EA2C02C882EFD84F22` (break `/Game/Blueprints/Character/F_CharacterData_Stance` (`/Game/Blueprints/Character/BP_Character.Active Stance` _array_element)))
      (`/Game/Blueprints/Character/BP_Character.Modify Character Action Pool` _array_element false _array_index 0)))
  (if (`/Game/Blueprints/Character/BP_Character.Moved This turn` (`local.character`))
    (set `/Game/Blueprints/Character/BP_Character.Moved This turn` false (`local.character`)))
  (`/Game/Blueprints/Core/Combat/BP_CombatSystem.Process Hits` :`self` (`self.Combat System`) :`Impact Data` (make `/Game/Blueprints/Core/Combat/Actions/Utility/F_ActionImpact` _returnvalue _returnvalue) :`character Ovveride` (`local.character`))
  (`/Game/Blueprints/Character/BP_Character.Modify Current Tokens` (`local.character`) _returnvalue "NewEnumerator6"))

(fn `UserConstructionScript`)