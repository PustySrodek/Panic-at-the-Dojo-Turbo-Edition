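; Combat action component that builds forced-movement push and pull paths on the tile grid, one chosen tile per call.
; Each step uses Manhattan distance from the attacker to exclude wrong-direction tiles, then marks valid adjacent tiles as candidates via grid tile states, skipping occupied, unwalkable or blocked ones.
; It returns an empty array until length, lack of candidates, certain tile or obstacle types, or an up-to confirmation ends the path.
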(fn `Get Distance to Target`
  (params (`Target Index` :type "IntPoint Structure"))
  (returns (NewParam :type Integer))
  (bind (_x _y) (break `IntPoint` `Target Index`))
  (bind (_x_2 _y_2) (break `IntPoint` (`self.Attacker Index`)))
  (return (+ (`KismetMathLibrary.Abs_Int` (- _x_2 _x)) (`KismetMathLibrary.Abs_Int` (- _y_2 _y)))))

(fn `initialize Push`
  (params (`Attacker Index` :type "IntPoint Structure") (`Path Length` :type Integer) (`Combat System` :type "/Game/Blueprints/Core/Combat/BP_CombatSystem Object Reference") (`Attacked Index` :type "IntPoint Structure"))
  (set `self.Attacker Index` `Attacker Index`)
  (set `self.Path Length` `Path Length`)
  (set `self.Combat System` `Combat System`)
  (bind _output_get (set `self.Target Index` `Attacked Index`))
  (set `self.Distance to Target` (`self.Get Distance to Target` _output_get)))

(fn `Set Pull Path`
  (params (`Target Index` :type "IntPoint Structure") (`Is Up to?` :type Boolean))
  (returns (Path :type "Array of IntPoint Structure"))
  (bind _grid_ref (`/Game/Blueprints/Core/Combat/BP_CombatSystem.Grid Ref` (`self.Combat System`)))
  (bind _grid_ref_2 (`/Game/Blueprints/Core/Combat/BP_CombatSystem.Grid Ref` (`self.Combat System`)))
  (bind (_index _tiletype _tiletransform _tilestate _unitontile _obstacles) (break `/Game/Blueprints/Grid/F_TileData` (`BlueprintMapLibrary.Map_Find` (`/Game/Blueprints/Grid/BP_Grid.Grid Tiles Data` (`/Game/Blueprints/Core/Combat/BP_CombatSystem.Grid Ref` (`self.Combat System`))) (`local.Target Index`))))
  (set `self.Target Index` `Target Index`)
  (if (not `Is Up to?`)
    (`/Game/Blueprints/Grid/BP_Grid.Clear All States from Tiles` _grid_ref_2 "NewEnumerator5")
    (`/Game/Blueprints/Grid/BP_Grid.Clear All States from Tiles` _grid_ref_2 "NewEnumerator8")
    (`/Game/Blueprints/Grid/BP_Grid.Add State to Tile` (`/Game/Blueprints/Core/Combat/BP_CombatSystem.Grid Ref` (`self.Combat System`)) (`local.Target Index`) "NewEnumerator7")
    (`|ExecutionSequence`
      (:`then_0`
        (bind _indexes_in_range (`/Game/Blueprints/Core/Combat/BP_CombatSystem.Get Action Range` (`self.Combat System`) (make `/Game/Blueprints/Core/Combat/Actions/Utility/F_ActionDataCast` "NewEnumerator2" (make `IntPoint` (`self.Distance to Target`) (+ (`self.Distance to Target`) 2)) false true 0.0 0.0) (`self.Attacker Index`)))
        (for _array_element _indexes_in_range
          (`/Game/Blueprints/Grid/BP_Grid.Add State to Tile` (`/Game/Blueprints/Core/Combat/BP_CombatSystem.Grid Ref` (`self.Combat System`)) _array_element "NewEnumerator8")))
      (:`then_1`
        (bind _indexes_in_range_2 (`/Game/Blueprints/Core/Combat/BP_CombatSystem.Get Action Range` (`self.Combat System`) (make `/Game/Blueprints/Core/Combat/Actions/Utility/F_ActionDataCast` (select `bool` (== (`self.Distance to Target`) 1) :`false` "NewEnumerator5" :`true` "NewEnumerator2" :!type "/Game/Blueprints/Core/Combat/Actions/Utility/Enum_RangePattern Enum") (make `IntPoint` 1 1) false true 0.0 0.0 0 true) (`self.Target Index`)))
        (for _array_element_2 _indexes_in_range_2
          (if (`self.Validate Range Index` _array_element_2)
            (`/Game/Blueprints/Grid/BP_Grid.Add State to Tile` (`/Game/Blueprints/Core/Combat/BP_CombatSystem.Grid Ref` (`self.Combat System`)) _array_element_2 "NewEnumerator5"))))
      (:`then_2`
        (bind _returnvalue (`KismetArrayLibrary.Array_Add` (`self.Path`) (`local.Target Index`)))
        (bind _indexe (`/Game/Blueprints/Grid/BP_Grid.Get All Tiles With State` (`/Game/Blueprints/Core/Combat/BP_CombatSystem.Grid Ref` (`self.Combat System`)) "NewEnumerator5"))
        (if (or (`KismetArrayLibrary.Array_IsEmpty` _indexe) (== _returnvalue (`self.Path Length`)) (`|EnumEquality` _tiletype "NewEnumerator6") (and (`.ReturnValue` (`BlueprintMapLibrary.Map_Find` _obstacles "NewEnumerator12")) (!= (`KismetArrayLibrary.Array_Length` (`self.Path`)) 1)))
          (`/Game/Blueprints/Grid/BP_Grid.Clear All States from Tiles` _grid_ref "NewEnumerator5" :!label _label)
          (`/Game/Blueprints/Grid/BP_Grid.Clear All States from Tiles` _grid_ref "NewEnumerator8")
          (`/Game/Blueprints/Grid/BP_Grid.Clear All States from Tiles` _grid_ref "NewEnumerator7")
          (return (`self.Path`))
          (else
            (set `self.Distance to Target` (`KismetMathLibrary.Min` (- (`self.Distance to Target`) 1) 1))
            (return (`|MakeArray`))))))
    (elif (`KismetArrayLibrary.Array_Contains` (`.TileState_15_2CD077A14CF44985E0DDB1AF1B2DA5B7` (break `/Game/Blueprints/Grid/F_TileData` (`BlueprintMapLibrary.Map_Find` (`/Game/Blueprints/Grid/BP_Grid.Grid Tiles Data` (`/Game/Blueprints/Core/Combat/BP_CombatSystem.Grid Ref` (`self.Combat System`))) (`local.Target Index`)))) "NewEnumerator7")
      (goto _label))))

(fn `Set Push Path`
  (params (`Target Index` :type "IntPoint Structure") (`Is Up to?` :type Boolean))
  (returns (Path :type "Array of IntPoint Structure"))
  (bind _grid_ref (`/Game/Blueprints/Core/Combat/BP_CombatSystem.Grid Ref` (`self.Combat System`)))
  (bind _grid_ref_2 (`/Game/Blueprints/Core/Combat/BP_CombatSystem.Grid Ref` (`self.Combat System`)))
  (bind (_index _tiletype _tiletransform _tilestate _unitontile _obstacles) (break `/Game/Blueprints/Grid/F_TileData` (`BlueprintMapLibrary.Map_Find` (`/Game/Blueprints/Grid/BP_Grid.Grid Tiles Data` (`/Game/Blueprints/Core/Combat/BP_CombatSystem.Grid Ref` (`self.Combat System`))) (`local.Target Index`))))
  (set `self.Target Index` `Target Index`)
  (if (not `Is Up to?`)
    (`/Game/Blueprints/Grid/BP_Grid.Clear All States from Tiles` _grid_ref_2 "NewEnumerator5")
    (`/Game/Blueprints/Grid/BP_Grid.Clear All States from Tiles` _grid_ref_2 "NewEnumerator8")
    (`/Game/Blueprints/Grid/BP_Grid.Add State to Tile` (`/Game/Blueprints/Core/Combat/BP_CombatSystem.Grid Ref` (`self.Combat System`)) (`local.Target Index`) "NewEnumerator7")
    (`|ExecutionSequence`
      (:`then_0`
        (bind _indexes_in_range (`/Game/Blueprints/Core/Combat/BP_CombatSystem.Get Action Range` (`self.Combat System`) (make `/Game/Blueprints/Core/Combat/Actions/Utility/F_ActionDataCast` "NewEnumerator2" (make `IntPoint` 0 (`self.Distance to Target`)) false true 0.0 0.0) (`self.Attacker Index`)))
        (for _array_element _indexes_in_range
          (`/Game/Blueprints/Grid/BP_Grid.Add State to Tile` (`/Game/Blueprints/Core/Combat/BP_CombatSystem.Grid Ref` (`self.Combat System`)) _array_element "NewEnumerator8")))
      (:`then_1`
        (bind _indexes_in_range_2 (`/Game/Blueprints/Core/Combat/BP_CombatSystem.Get Action Range` (`self.Combat System`) (make `/Game/Blueprints/Core/Combat/Actions/Utility/F_ActionDataCast` "NewEnumerator2" (make `IntPoint` 1 1) false true 0.0 0.0 0 true) (`self.Target Index`)))
        (for _array_element_2 _indexes_in_range_2
          (if (`self.Validate Range Index` _array_element_2)
            (`/Game/Blueprints/Grid/BP_Grid.Add State to Tile` (`/Game/Blueprints/Core/Combat/BP_CombatSystem.Grid Ref` (`self.Combat System`)) _array_element_2 "NewEnumerator5"))))
      (:`then_2`
        (bind _returnvalue (`KismetArrayLibrary.Array_Add` (`self.Path`) (`local.Target Index`)))
        (bind _indexe (`/Game/Blueprints/Grid/BP_Grid.Get All Tiles With State` (`/Game/Blueprints/Core/Combat/BP_CombatSystem.Grid Ref` (`self.Combat System`)) "NewEnumerator5"))
        (if (or (`KismetArrayLibrary.Array_IsEmpty` _indexe) (== _returnvalue (`self.Path Length`)) (`|EnumEquality` _tiletype "NewEnumerator6") (and (`.ReturnValue` (`BlueprintMapLibrary.Map_Find` _obstacles "NewEnumerator12")) (!= (`KismetArrayLibrary.Array_Length` (`self.Path`)) 1)))
          (`/Game/Blueprints/Grid/BP_Grid.Clear All States from Tiles` _grid_ref "NewEnumerator5" :!label _label)
          (`/Game/Blueprints/Grid/BP_Grid.Clear All States from Tiles` _grid_ref "NewEnumerator8")
          (`/Game/Blueprints/Grid/BP_Grid.Clear All States from Tiles` _grid_ref "NewEnumerator7")
          (return (`self.Path`))
          (else
            (set `self.Distance to Target` (+ (`self.Distance to Target`) 1))
            (return (`|MakeArray`))))))
    (elif (`KismetArrayLibrary.Array_Contains` (`.TileState_15_2CD077A14CF44985E0DDB1AF1B2DA5B7` (break `/Game/Blueprints/Grid/F_TileData` (`BlueprintMapLibrary.Map_Find` (`/Game/Blueprints/Grid/BP_Grid.Grid Tiles Data` (`/Game/Blueprints/Core/Combat/BP_CombatSystem.Grid Ref` (`self.Combat System`))) (`local.Target Index`)))) "NewEnumerator0")
      (goto _label))))

(fn `Validate Range Index`
  (params (Index :type "IntPoint Structure"))
  (returns (ReturnValue :type Boolean))
  (bind (_index _tiletype _tiletransform _tilestate _unitontile _obstacles) (break `/Game/Blueprints/Grid/F_TileData` (`BlueprintMapLibrary.Map_Find` (`/Game/Blueprints/Grid/BP_Grid.Grid Tiles Data` (`/Game/Blueprints/Core/Combat/BP_CombatSystem.Grid Ref` (`self.Combat System`))) Index)))
  (return (not (or (`KismetArrayLibrary.Array_Contains` _tilestate "NewEnumerator8") (`KismetArrayLibrary.Array_Contains` _tilestate "NewEnumerator7") (`KismetSystemLibrary.IsValid` _unitontile) (not (`/Game/Blueprints/Grid/BP_Grid.Is Tile Walkable` (`/Game/Blueprints/Core/Combat/BP_CombatSystem.Grid Ref` (`self.Combat System`)) (`local.Index`))) (`.ReturnValue` (`BlueprintMapLibrary.Map_Find` _obstacles "NewEnumerator10"))))))