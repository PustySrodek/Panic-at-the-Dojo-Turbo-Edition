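; Actor that runs one grid-based unit action for the active cast (combat) or perform (out-of-combat) command, destroying itself when that command is killed.
; It disables combat-menu buttons, spawns debug shapes toward attacked tiles, and on the first one's completion processes hits through CombatSystem.
; It then re-enables the menu, spends the unit's selected die and finishes the command.
; Helpers, uncalled here, validate tiles and resolve targets, using a picker widget unless exactly one exists.
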(event `self.ReceiveBeginPlay`
  (bind (_index _tiletype _tiletransform _tilestate _unitontile) (break `/Game/Blueprints/Grid/F_TileData` (`BlueprintMapLibrary.Map_Find` (`/Game/Blueprints/Grid/BP_Grid.Grid Tiles Data` (`self.Grid`)) (`self.Origin Index`))))
  (bind _returnvalue (`GameplayStatics.GetActorOfClass` "/Game/Blueprints/Core/Commands/BP_PlayerCommands.BP_PlayerCommands_C"))
  (bind _output_get (set `self.Player Commands` _returnvalue))
  (bind _output_get_2 (set `self.Combat System` (`/Game/Blueprints/Core/Commands/BP_PlayerCommands.Combat System` _output_get)))
  (set `self.Grid` (`/Game/Blueprints/Core/Commands/BP_PlayerCommands.Grid` _output_get))
  (if (`/Game/Blueprints/Core/Combat/BP_CombatSystem.Is In Combat` _output_get_2)
    (bind _asccommand_cast_action (cast `/Game/Blueprints/Core/Commands/Combat/CCommand_CastAction` (`/Game/Blueprints/Core/Commands/BP_PlayerCommands.Selected Left Click` (`self.Player Commands`))))
    (bind _output_get_3 (set `self.Command` _asccommand_cast_action))
    (add `/Game/Blueprints/Core/Commands/Combat/CCommand_CastAction.On Command Kill` _output_get_3 (delegate `On Command Death`))
    (else
      (bind _ascommand_perform_action (cast `/Game/Blueprints/Core/Commands/Characters/Command_PerformAction` (`/Game/Blueprints/Core/Commands/BP_PlayerCommands.Selected Right Click` (`self.Player Commands`))))
      (bind _output_get_4 (set `self.[Debug] Command` _ascommand_perform_action))
      (add `/Game/Blueprints/Core/Commands/Characters/Command_PerformAction.On Command Kill` _output_get_4 (delegate `On Command Death`))))
  (`/Engine/EditorBlueprintResources/StandardMacros.IsValid` _unitontile
    (:`Is Valid`
      (`/Game/Blueprints/Character/BP_Character.Do Action` _unitontile (`self.Target index`))
      (`self.Do The Action`))))

(event `On Command Death`
  (`self.K2_DestroyActor`))

(event `Do The Action`
  (bind (_meshsize _mesh _flatmesh _meshmaterial) (break `/Game/Blueprints/Grid/F_GridShapeData` (`/Game/Blueprints/Grid/BP_Grid.Out Row` (`self.Grid`))))
  (`self.Enable Stage` true)
  (for (_array_element _array_index) (`self.Attacked Indexes`)
    (bind _returnvalue (`|SpawnActorFromClass` "/Game/Blueprints/Core/Combat/Actions/Components/BP_DebugAnimShape.BP_DebugAnimShape_C" (`KismetMathLibrary.MakeTransform` (0.0 0.0 0.0)) "AlwaysSpawn" "MultiplyWithRoot" null _mesh _meshmaterial (struct :`R` 0.401042 :`A` 1.0) (`.TileTransform_9_C8B49F424080CB25DC8191A7EE85CF00` (break `/Game/Blueprints/Grid/F_TileData` (`BlueprintMapLibrary.Map_Find` (`/Game/Blueprints/Grid/BP_Grid.Grid Tiles Data` (`self.Grid`)) (`self.Origin Index`)))) (`.TileTransform_9_C8B49F424080CB25DC8191A7EE85CF00` (break `/Game/Blueprints/Grid/F_TileData` (`BlueprintMapLibrary.Map_Find` (`/Game/Blueprints/Grid/BP_Grid.Grid Tiles Data` (`self.Grid`)) _array_element))) null))
    (if (== _array_index 0)
      (add `/Game/Blueprints/Core/Combat/Actions/Components/BP_DebugAnimShape.On Debug Anim Completed` _returnvalue (delegate `On Debug anim Completed`)))))

(event `On Debug anim Completed`
  (params (NewParam :type "/Game/Blueprints/Core/Combat/Actions/Components/BP_DebugAnimShape Object Reference"))
  (`self.Action Logic`)
  (`self.Enable Stage` false)
  (`self.Action Finishing`))

(event `Action Finishing`
  (bind __debug__command (`self.[Debug] Command`))
  (bind _command (`self.Command`))
  (bind (_index _tiletype _tiletransform _tilestate _unitontile) (break `/Game/Blueprints/Grid/F_TileData` (`BlueprintMapLibrary.Map_Find` (`/Game/Blueprints/Grid/BP_Grid.Grid Tiles Data` (`self.Grid`)) (`self.Origin Index`))))
  (`/Engine/EditorBlueprintResources/StandardMacros.IsValid` _unitontile
    (:`Is Valid`
      (`/Game/Blueprints/Character/BP_Character.Modify Character Action Pool` _unitontile false (`/Game/Blueprints/Character/BP_Character.Selected Die Index` _unitontile) 0)
      (`/Game/Blueprints/Character/BP_Character.Set Selected Number and Index` _unitontile 0 -1))
    (:`Is Not Valid`
      _))
  (`/Engine/EditorBlueprintResources/StandardMacros.IsValid` __debug__command
    (:`Is Valid`
      (`/Game/Blueprints/Core/Commands/Characters/Command_PerformAction.Finish Action` __debug__command))
    (:`Is Not Valid`
      (`/Engine/EditorBlueprintResources/StandardMacros.IsValid` _command
        (:`Is Valid`
          (`/Game/Blueprints/Core/Commands/Combat/CCommand_CastAction.Finish Action` _command))))))

(event `Player Picked Character`
  (params (Character :type "/Game/Blueprints/Character/BP_Character Object Reference"))
  (bind _enemy_picker (`self.Enemy Picker`))
  (`/Engine/EditorBlueprintResources/StandardMacros.IsValid` _enemy_picker
    (:`Is Valid`
      (`Widget.RemoveFromParent` _enemy_picker))))

(event `Player Picked Obstacle`
  (params (Obstacle :type "/Game/Blueprints/Core/Combat/Obstacles/ObstacleClasses/BP_Obstacle Object Reference"))
  (bind _enemy_picker (`self.Enemy Picker`))
  (`/Engine/EditorBlueprintResources/StandardMacros.IsValid` _enemy_picker
    (:`Is Valid`
      (`Widget.RemoveFromParent` _enemy_picker))))

(fn `Action Logic`
  (bind _damagevalue (break `/Game/Blueprints/Core/Combat/Actions/Utility/F_ActionImpact` (`.ImpactData_16_2A6944184758C49277D58CA8095E19F1` (break `/Game/Blueprints/Core/Combat/Actions/Utility/F_ActionsData` (`self.Action Data`)))))
  (`/Game/Blueprints/Core/Combat/BP_CombatSystem.Process Hits` (`self.Combat System`) (`self.Attacked Indexes`) (make `/Game/Blueprints/Core/Combat/Actions/Utility/F_ActionImpact` _damagevalue _damagevalue) null))

(fn `Choose Specify Target Method`
  (if (!= (`KismetArrayLibrary.Array_Length` (`self.Possible Targets`)) 1)
    (`self.Create Enemy Picker` (`self.Possible Targets`))
    (else
      (`self.Specify Target` (`|GetArrayItem` (`self.Possible Targets`))))))

(fn `Create Enemy Picker`
  (params (Targets :type "Array of Object Object Reference"))
  (bind _enemy_picker (`self.Enemy Picker`))
  (bind _returnvalue (`|CreateWidget` "/Game/Blueprints/Core/Combat/Actions/Components/Widgets/TagetPickers/TP_DefaultEnemy.TP_DefaultEnemy_C" (`GameplayStatics.GetPlayerController` 0) Targets))
  (bind _output_get (set `self.Enemy Picker` _returnvalue))
  (`UserWidget.AddToPlayerScreen` _output_get 0)
  (add `/Game/Blueprints/Core/Combat/Actions/Components/Widgets/TagetPickers/TP_DefaultEnemy.On Obstacle Picked` _enemy_picker (`|CreateDelegate` :!event `Player Picked Obstacle`))
  (add `/Game/Blueprints/Core/Combat/Actions/Components/Widgets/TagetPickers/TP_DefaultEnemy.On Character Picked` _enemy_picker (`|CreateDelegate` :!event `Player Picked Character`)))

(fn `Enable Stage`
  (params (`Is Enabled` :type Boolean))
  (bind _combat_menu (`/Game/Blueprints/Core/Commands/BP_PlayerCommands.Combat Menu` (`self.Player Commands`)))
  (set `self.Is Stage Finished` (not `Is Enabled`))
  (`/Engine/EditorBlueprintResources/StandardMacros.IsValid` _combat_menu
    (:`Is Valid`
      (for _array_element (`PanelWidget.GetAllChildren` (`/Game/Blueprints/HUD/Debug_Menu/Buttons/ButtonList_Actions.ActionPanel` (`/Game/Blueprints/HUD/Combat_Menu/WBP_CombatMenu.ButtonList_Actions` _combat_menu)))
        (`Widget.SetIsEnabled` _array_element (`self.Is Stage Finished`)))
      (for _array_element_2 (`PanelWidget.GetAllChildren` (`/Game/Blueprints/HUD/Debug_Menu/Buttons/ButtonList_ActionDice.DicePanel` (`/Game/Blueprints/HUD/Combat_Menu/WBP_CombatMenu.ButtonList_ActionDice` _combat_menu)))
        (`Widget.SetIsEnabled` _array_element_2 (`self.Is Stage Finished`))))
    (:`Is Not Valid`
      (`KismetSystemLibrary.PrintString` "Combat Menu not valid"))))

(fn `Get Enemy Obstacles`
  (params (Obstacles :type "Map of /Game/Blueprints/Core/Combat/Obstacles/Utility/Enum_Obstacles Enum to /Game/Blueprints/Core/Combat/Obstacles/ObstacleClasses/BP_Obstacle Object Reference (by ref)"))
  (returns (`Enemy Obstacles` :type "Array of /Game/Blueprints/Core/Combat/Obstacles/ObstacleClasses/BP_Obstacle Object Reference"))
  (locals (`Obstacle Array` :type "Array of /Game/Blueprints/Core/Combat/Obstacles/ObstacleClasses/BP_Obstacle Object Reference"))
  (if (not (`BlueprintMapLibrary.Map_IsEmpty` Obstacles))
    (`|ExecutionSequence`
      (:`then_0`
        (bind _keys (`BlueprintMapLibrary.Map_Keys` (`local.Obstacles`)))
        (for _array_element _keys
          (if (or (`|EnumEquality` _array_element "NewEnumerator11") (`|EnumEquality` _array_element "NewEnumerator10") (`|EnumEquality` _array_element "NewEnumerator12"))
            (`KismetArrayLibrary.Array_Add` (`local.Obstacle Array`) (`BlueprintMapLibrary.Map_Find` (`local.Obstacles`) _array_element)))))
      (:`then_1`
        (return (`local.Obstacle Array`))))
    (else
      (return (`|MakeArray`)))))

(fn `Is Target Index Valid `
  (returns (`Return Value` :type Boolean))
  (bind (_index _tiletype _tiletransform _tilestate _unitontile) (break `/Game/Blueprints/Grid/F_TileData` (`BlueprintMapLibrary.Map_Find` (`/Game/Blueprints/Grid/BP_Grid.Grid Tiles Data` (`self.Grid`)) (`self.Target index`))))
  (return (and (`KismetArrayLibrary.Array_Contains` _tilestate "NewEnumerator5") (not (`KismetArrayLibrary.Array_Contains` _tilestate "NewEnumerator8")) (not (`KismetArrayLibrary.Array_Contains` _tilestate "NewEnumerator7")) (not (`KismetSystemLibrary.IsValid` _unitontile)))))

(fn `Set Possible Enemies`
  (returns (`No Possible Targets` :type Boolean))
  (bind (_index _tiletype _tiletransform _tilestate _unitontile _obstacles) (break `/Game/Blueprints/Grid/F_TileData` (`BlueprintMapLibrary.Map_Find` (`/Game/Blueprints/Grid/BP_Grid.Grid Tiles Data` (`self.Grid`)) (`self.Target index`))))
  (bind _enemy_obstacles (`self.Get Enemy Obstacles` _obstacles))
  (set `self.Possible Targets` _enemy_obstacles)
  (`/Engine/EditorBlueprintResources/StandardMacros.IsValid` _unitontile
    (:`Is Valid`
      (`KismetArrayLibrary.Array_Add` (`self.Possible Targets`) _unitontile))
    (:`Is Not Valid`
      _))
  (return (not (`KismetArrayLibrary.Array_IsEmpty` (`self.Possible Targets`)))))

(fn `Specify Target`
  (params (Target :type "Object Object Reference"))
  (locals (`Target Character` :type "/Game/Blueprints/Character/BP_Character Object Reference") (`Target Obstacle` :type "/Game/Blueprints/Core/Combat/Obstacles/ObstacleClasses/BP_Obstacle Object Reference"))
  (bind _target_obstacle (`local.Target Obstacle`))
  (bind _outactors (`GameplayStatics.GetAllActorsOfClass` "/Game/Blueprints/Character/BP_Character.BP_Character_C"))
  (for _array_element _outactors
    (if (`KismetStringLibrary.EqualEqual_StrStr` (`KismetSystemLibrary.GetObjectName` _array_element) (`KismetSystemLibrary.GetObjectName` (`local.Target`)))
      (set `local.Target Character` _array_element)
      (break)))
  (`/Engine/EditorBlueprintResources/StandardMacros.IsValid` (`local.Target Character`)
    (:`Is Valid`
      (`self.Player Picked Character` (`local.Target Character`)))
    (:`Is Not Valid`
      (bind _outactors_2 (`GameplayStatics.GetAllActorsOfClass` "/Game/Blueprints/Core/Combat/Obstacles/ObstacleClasses/BP_Obstacle.BP_Obstacle_C"))
      (for _array_element_2 _outactors_2
        (if (`KismetStringLibrary.EqualEqual_StrStr` (`KismetSystemLibrary.GetObjectName` _array_element_2) (`KismetSystemLibrary.GetObjectName` (`local.Target`)))
          (set `local.Target Obstacle` _array_element_2)
          (break)))
      (`/Engine/EditorBlueprintResources/StandardMacros.IsValid` _target_obstacle
        (:`Is Valid`
          (`self.Player Picked Obstacle` _target_obstacle))
        (:`Is Not Valid`
          (`KismetSystemLibrary.PrintString` "found no target"))))))

(fn `UserConstructionScript`)