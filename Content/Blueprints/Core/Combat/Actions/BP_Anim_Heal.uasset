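; BP_Anim_Heal is a combat action animation actor for the Heal action on the tile grid.
; On DotheAction it looks up the target tile in the grid data and moves itself to that tile's location.
; A Timeline then drives the scale and yaw rotation of its Scene component, and calls ActionAnimationFinished when it completes.
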(event `self.Do The Action`
  (bind _scene (`self.Scene`))
  (`self.K2_SetActorLocation` (.location (`.TileTransform_9_C8B49F424080CB25DC8191A7EE85CF00` (break `/Game/Blueprints/Grid/F_TileData` (`BlueprintMapLibrary.Map_Find` (`/Game/Blueprints/Grid/BP_Grid.Grid Tiles Data` (`self.Grid`)) (`self.Target indexes`))))))
  (bind (_direction _scale _rotation) (`Timeline|Timeline` :!via `PlayFromStart`)
    (:`Update`
      (`SceneComponent.SetRelativeScale3D` _scene _scale)
      (`SceneComponent.K2_SetRelativeRotation` _scene (`KismetMathLibrary.MakeRotator` 0.0 0.0 _rotation) false false))
    (:`Finished`
      (`self.Action Animation Finished`))))

(fn `UserConstructionScript`
  (`parent.UserConstructionScript`))