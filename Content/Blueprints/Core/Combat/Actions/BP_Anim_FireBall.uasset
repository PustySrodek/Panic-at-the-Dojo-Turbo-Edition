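; Fireball animation actor for a combat action on the tile grid, flying from the origin tile to the target tile.
; DotheAction snaps the actor to the origin tile and plays a timeline that drives location interpolation, scene scale and visibility.
; Float tracks are converted to booleans to toggle hidden states during flight.
; When the timeline finishes, it calls ActionAnimationFinished to signal completion.
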(event `self.Do The Action`
  (bind _grid_tiles_data (`/Game/Blueprints/Grid/BP_Grid.Grid Tiles Data` (`self.Grid`)))
  (`self.K2_SetActorLocation` (.location (`.TileTransform_9_C8B49F424080CB25DC8191A7EE85CF00` (break `/Game/Blueprints/Grid/F_TileData` (`BlueprintMapLibrary.Map_Find` (`/Game/Blueprints/Grid/BP_Grid.Grid Tiles Data` (`self.Grid`)) (`self.Origin Index`))))))
  (bind (_direction _scale _location_alpha _scene_hidden _ball_hidden) (`Timeline|Timeline` :!via `PlayFromStart`)
    (:`Update`
      (`SceneComponent.SetHiddenInGame` (`self.Scene`) (`KismetMathLibrary.Conv_IntToBool` (`KismetMathLibrary.FTrunc` _ball_hidden)) true)
      (`self.K2_SetActorLocation` (`KismetMathLibrary.VLerp` (.location (`.TileTransform_9_C8B49F424080CB25DC8191A7EE85CF00` (break `/Game/Blueprints/Grid/F_TileData` (`BlueprintMapLibrary.Map_Find` _grid_tiles_data (`self.Origin Index`))))) (.location (`.TileTransform_9_C8B49F424080CB25DC8191A7EE85CF00` (break `/Game/Blueprints/Grid/F_TileData` (`BlueprintMapLibrary.Map_Find` _grid_tiles_data (`self.Target indexes`))))) _location_alpha))
      (`SceneComponent.SetHiddenInGame` (`self.Scene`) (`KismetMathLibrary.Conv_IntToBool` (`KismetMathLibrary.FTrunc` _scene_hidden)) true)
      (`SceneComponent.SetRelativeScale3D` (`self.Scene`) _scale))
    (:`Finished`
      (`self.Action Animation Finished`))))

(fn `UserConstructionScript`
  (`parent.UserConstructionScript`))