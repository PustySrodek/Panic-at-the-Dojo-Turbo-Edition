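; Combat action Blueprint for movement that feeds the selected die number into the current character's tokens.
; ActionLogic passes the sum of the first token type's stored value and the selected die number to ModifyCurrentTokens on the CombatSystem's current character.
; DotheAction plays no animation of its own, only waiting briefly before calling ActionAnimationFinished.
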(event `self.Do The Action`
  (`KismetSystemLibrary.Delay` 0.2)
  (`self.Action Animation Finished`))

(fn `Action Logic`
  (bind _current_character (`/Game/Blueprints/Core/Combat/BP_CombatSystem.Current Character` (`self.Combat System`)))
  (bind (_canmovediagonaly _validtiletypes _basicactions _currenthealth _maxhealth _currentshield _maxshield _numberofhealthbars _tokens _actionpool _selecteddienumber) (break `/Game/Blueprints/Characters/F_CharacterData_Stats` (`.Stats_5_5DCC378E48218015EE4248AF0BBAB223` (break `/Game/Blueprints/Characters/F_CharacterData` (`/Game/Blueprints/Characters/BP_Character.Character Data` _current_character)))))
  (`/Game/Blueprints/Characters/BP_Character.Modify Current Tokens` _current_character (+ (`BlueprintMapLibrary.Map_Find` _tokens "NewEnumerator0") _selecteddienumber) "NewEnumerator0"))

(fn `UserConstructionScript`
  (`parent.UserConstructionScript`))