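; BP_AH_Damage is a combat action that deals damage on the grid, scaled by the current character's selected die number.
; DotheAction places the actor on the origin tile facing the target, plays a sword rotation and scale timeline, then signals completion.
; ActionLogic maps die numbers in pairs to stepped negative damage, capped from nine up, and passes it with a health modifier to CombatSystem.ProcessHits for the attacked tiles.
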(event `self.Do The Action`
  (bind _anim_scaleandrotation (`self.Anim_ScaleAndRotation`))
  (bind (_returnvalue_x _returnvalue_y) (`KismetMathLibrary.BreakVector2D` (`KismetMathLibrary.Conv_IntPointToVector2D` (`self.Target indexes`))))
  (bind (_returnvalue_x_2 _returnvalue_y_2) (`KismetMathLibrary.BreakVector2D` (`KismetMathLibrary.Conv_IntPointToVector2D` (`self.Origin Index`))))
  (`self.K2_SetActorLocationAndRotation` (.location (`.TileTransform_9_C8B49F424080CB25DC8191A7EE85CF00` (break `/Game/Blueprints/Grid/F_TileData` (`BlueprintMapLibrary.Map_Find` (`/Game/Blueprints/Grid/BP_Grid.Grid Tiles Data` (`self.Grid`)) (`self.Origin Index`))))) (`KismetMathLibrary.FindLookAtRotation` (`KismetMathLibrary.MakeVector` _returnvalue_x_2 _returnvalue_y_2) (`KismetMathLibrary.MakeVector` _returnvalue_x _returnvalue_y)))
  (bind (_direction _rotation_y _scale) (`Timeline|Sword Anim` :!via `PlayFromStart`)
    (:`Update`
      (`SceneComponent.K2_SetRelativeRotation` _anim_scaleandrotation (`KismetMathLibrary.MakeRotator` 0.0 _rotation_y) false false)
      (`SceneComponent.SetRelativeScale3D` _anim_scaleandrotation (`KismetMathLibrary.Conv_DoubleToVector` _scale)))
    (:`Finished`
      (`self.Action Animation Finished`))))

(fn `Action Logic`
  (locals (`Damage Value` :type Integer))
  (bind (_canmovediagonaly _validtiletypes _basicactions _currenthealth _maxhealth _currentshield _maxshield _numberofhealthbars _tokens _actionpool _selecteddienumber) (break `/Game/Blueprints/Characters/F_CharacterData_Stats` (`.Stats_5_5DCC378E48218015EE4248AF0BBAB223` (break `/Game/Blueprints/Characters/F_CharacterData` (`/Game/Blueprints/Characters/BP_Character.Character Data` (`/Game/Blueprints/Core/Combat/BP_CombatSystem.Current Character` (`self.Combat System`)))))))
  (if (>= _selecteddienumber 9)
    (set `local.Damage Value` -5)
    (else
      (switch `int` _selecteddienumber
        (:`1`
          (set `local.Damage Value` -1 :!label _label))
        (:`2`
          (goto _label))
        (:`3`
          (set `local.Damage Value` -2 :!label _label_2))
        (:`4`
          (goto _label_2))
        (:`5`
          (set `local.Damage Value` -3 :!label _label_3))
        (:`6`
          (goto _label_3))
        (:`7`
          (set `local.Damage Value` -4 :!label _label_4))
        (:`8`
          (goto _label_4)))))
  (`/Game/Blueprints/Core/Combat/BP_CombatSystem.Process Hits` (`self.Combat System`) (`self.Attacked Indexes`) (make `/Game/Blueprints/Core/Combat/Actions/Utility/F_ActionImpact` (`local.Damage Value`) (`/Game/Blueprints/Core/Combat/BP_CombatSystem.Get Health Modifier` (`self.Combat System`) (`local.Damage Value`)))))

(fn `UserConstructionScript`
  (`parent.UserConstructionScript`))