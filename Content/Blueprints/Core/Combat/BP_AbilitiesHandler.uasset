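; BP_AbilitiesHandler rolls dice for a character to build the action pool of its active stance.
; RollDiceForCharacter looks up the data for the stance's Form and passes its dice values to SetActionPoolFromDice.
; Any Numbers in that form data are then added through ModifyCharacterActionPool.
; Debug prints show the form, the dice and the pool, which reprints after each added number.
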(fn `Roll Dice For Character`
  (params (Character :type "/Game/Blueprints/Character/BP_Character Object Reference"))
  (bind (_actionpool _range _archetypes _style _form) (break `/Game/Blueprints/Character/F_CharacterData_Stance` (`/Game/Blueprints/Character/BP_Character.Active Stance` Character)))
  (`KismetSystemLibrary.PrintString` (`|GetEnumeratorNameAsString` _form))
  (bind _out_row (`/Game/Blueprints/Core/Combat/Utility/BFL_Combat.Get Form Data From Form` _form))
  (bind (_name _altnames _dice _numbers) (break `/Game/Blueprints/CharacterCreation/Forms/F_FormsData` _out_row))
  (bind _values (`BlueprintMapLibrary.Map_Values` _dice))
  (for _array_element _values
    (`KismetSystemLibrary.PrintString` (`KismetStringLibrary.Conv_IntToString` _array_element)))
  (`/Game/Blueprints/Character/BP_Character.Set Action Pool From Dice` (`local.Character`) _values)
  (if (`KismetArrayLibrary.Array_IsEmpty` _numbers)
    (for _array_element_2 (`.ActionPool_5_B5573866494C04EA2C02C882EFD84F22` (break `/Game/Blueprints/Character/F_CharacterData_Stance` (`/Game/Blueprints/Character/BP_Character.Active Stance` (`local.Character`)))) :!label _label
      (`KismetSystemLibrary.PrintString` (`KismetStringLibrary.Conv_IntToString` _array_element_2)))
    (else
      (for _array_element_3 _numbers
        (`/Game/Blueprints/Character/BP_Character.Modify Character Action Pool` (`local.Character`) true _array_element_3 0)
        (goto _label)))))

(fn `UserConstructionScript`)