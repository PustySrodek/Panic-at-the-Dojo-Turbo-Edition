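; BP_Camera is a player-controlled spring-arm camera that moves, zooms, rotates and tilts, using the ICM_TurnBase Enhanced Input mapping context it adds on BeginPlay.
; Input events only update target values: planar location along the camera's flattened axes, arm length, yaw, and pitch (named Pan).
; Tick interpolates the actor and spring arm toward these targets for smooth motion.
; Zoom and pitch are clamped, while movement has no bounds.
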(event `self.ReceiveBeginPlay`
  ;[0 0 0] Camera initialization
  ;;[0.1562 0.1562 0.1562 0.4] Initialize the camera controls
  (bind _asbp_pcpat_d (cast `/Game/Blueprints/Core/Player/BP_PCPatD` (`GameplayStatics.GetPlayerController` 0)))
  (`EnhancedInputSubsystemInterface.AddMappingContext` (pcsubsystem `EnhancedInputLocalPlayerSubsystem` _asbp_pcpat_d) "/Game/Inputs/ICM_TurnBase.ICM_TurnBase" 0 (struct))
  ;;[0.1562 0.1562 0.1562 0.4] Initialize camera postion
  (set `self.Desiered Location` (`self.K2_GetActorLocation`))
  (set `self.Desiered Zoom` (`SpringArmComponent.TargetArmLength` (`self.SpringArm`))))

(event `self.ReceiveTick`
  (params (DeltaSeconds :type "Float (single-precision)"))
  (bind (_desiered_rotation_roll _desiered_rotation_pitch _desiered_rotation_yaw) (`KismetMathLibrary.BreakRotator` (`self.Desiered Rotation`)))
  (bind _springarm (`self.SpringArm`))
  (bind (_desired_pan_roll _desired_pan_pitch) (`KismetMathLibrary.BreakRotator` (`self.Desired Pan`)))
  (bind (_returnvalue_roll _returnvalue_pitch _returnvalue_yaw) (`KismetMathLibrary.BreakRotator` (`KismetMathLibrary.RInterpTo` (`self.K2_GetActorRotation`) (`KismetMathLibrary.MakeRotator` 0.0 _desired_pan_pitch _desiered_rotation_yaw) DeltaSeconds 5.0)))
  ;[0 0 0] Camera Zoom Logic
  ;;[0.1562 0.1562 0.1562 0.4] Whenever the player zooms in, this smoothes the zoom. This effect can be modified by simply changing
  ;; the inerp speed value in FInterp function
  (set `SpringArmComponent.TargetArmLength` (`KismetMathLibrary.FInterpTo` (`SpringArmComponent.TargetArmLength` _springarm) (`self.Desiered Zoom`) DeltaSeconds 4.0) _springarm)
  ;[0 0 0] Camera Movement Logic
  ;;[0.1562 0.1562 0.1562 0.4] Whenever the player moves the camera, this smoothes this movement. This effect can be modified by simply changing the inerp speed value in VInterp function
  (`self.K2_SetActorLocation` (`KismetMathLibrary.VInterpTo` (`self.K2_GetActorLocation`) (`self.Desiered Location`) DeltaSeconds 6.0))
  ;[0 0 0] Camera Rotation Logic
  ;;[0.1562 0.1562 0.1562 0.4] Whenever the player rotates the camera, this smoothes this rotation. This effect can be modified by simply changing the inerp speed value in RInterp function
  (`self.K2_SetActorRelativeRotation` (`KismetMathLibrary.MakeRotator` 0.0 _returnvalue_pitch _returnvalue_yaw)))

(event `EnhancedInput|/Game/Inputs/IA_CameraMove`
  (params (ActionValue :type "Vector2D Structure") (ElapsedSeconds :type "Float (double-precision)") (TriggeredSeconds :type "Float (double-precision)") (InputAction :type "InputAction Object Reference" :default "/Game/Inputs/IA_CameraMove.IA_CameraMove"))
  (bind (_returnvalue_x _returnvalue_y) (`KismetMathLibrary.BreakVector2D` (`KismetMathLibrary.Normal2D` ActionValue)))
  (bind (_returnvalue_x_2 _returnvalue_y_2) (`KismetMathLibrary.BreakVector` (`self.GetActorRightVector`)))
  (bind (_returnvalue_x_3 _returnvalue_y_3) (`KismetMathLibrary.BreakVector` (`self.GetActorForwardVector`)))
  ;[0 0 0] Camera Movement Logic
  ;;[0.1562 0.1562 0.1562 0.4] Core of Camera Movement. The speed of camera movement can simply be modified by changing the camera move speed variable. The camera has no set boundries for now
  (:`Triggered`
    (set `self.Desiered Location` (+ (* (`KismetMathLibrary.MakeVector` _returnvalue_x_3 _returnvalue_y_3) (* (`self.Camera Move Speed`) _returnvalue_x)) (`self.Desiered Location`) (* (* _returnvalue_y (`self.Camera Move Speed`)) (`KismetMathLibrary.MakeVector` _returnvalue_x_2 _returnvalue_y_2))))))

(event `EnhancedInput|/Game/Inputs/IA_CameraRotate`
  (params (ActionValue :type "Float (double-precision)") (ElapsedSeconds :type "Float (double-precision)") (TriggeredSeconds :type "Float (double-precision)") (InputAction :type "InputAction Object Reference" :default "/Game/Inputs/IA_CameraRotate.IA_CameraRotate"))
  ;[0 0 0] Camera Rotation Logic
  ;;[0.1562 0.1562 0.1562 0.4] Core of Camera Rotation. The speed of the rotation can simply be modified by changing the camera rotation speed variable.
  (:`Triggered`
    (set `self.Desiered Rotation` (`KismetMathLibrary.ComposeRotators` (`self.Desiered Rotation`) (`KismetMathLibrary.MakeRotator` 0.0 0.0 (* ActionValue (`self.Rotation Speed`)))))))

(event `EnhancedInput|/Game/Inputs/IA_CameraZoom`
  (params (ActionValue :type "Float (double-precision)") (ElapsedSeconds :type "Float (double-precision)") (TriggeredSeconds :type "Float (double-precision)") (InputAction :type "InputAction Object Reference" :default "/Game/Inputs/IA_CameraZoom.IA_CameraZoom"))
  ;[0 0 0] Camera Zoom Logic
  ;;[0.1562 0.1562 0.1562 0.4] Core of camera zoom. The quantity of levels the zoom goes through and thus how fast it is can be changed by multiplying
  ;; the action value  by diffent numbers. The higher the number the zoom goes through less levels.
  ;;
  ;; The Maxium and minimum levels of zoom can be changed in the clamp function
  (:`Triggered`
    (set `self.Desiered Zoom` (`KismetMathLibrary.FClamp` (+ (`self.Desiered Zoom`) (* ActionValue (`self.Zoom Speed`))) 100.0 1500.0))))

(event `EnhancedInput|/Game/Inputs/IA_CameraPan`
  (params (ActionValue :type "Float (double-precision)") (ElapsedSeconds :type "Float (double-precision)") (TriggeredSeconds :type "Float (double-precision)") (InputAction :type "InputAction Object Reference" :default "/Game/Inputs/IA_CameraPan.IA_CameraPan"))
  (bind (_returnvalue_roll _returnvalue_pitch) (`KismetMathLibrary.BreakRotator` (`KismetMathLibrary.ComposeRotators` (`self.Desired Pan`) (`KismetMathLibrary.MakeRotator` 0.0 (* ActionValue (`self.Pan Speed`))))))
  (:`Triggered`
    (set `self.Desired Pan` (`KismetMathLibrary.MakeRotator` 0.0 (`KismetMathLibrary.FClamp` _returnvalue_pitch -49.0 40.0)))))

(fn `UserConstructionScript`)