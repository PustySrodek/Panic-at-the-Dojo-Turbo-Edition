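; Grid-based, turn-based combat character, defaulting to a warrior mesh, with health bars, shield, armor, tokens and team color.
; FollowPath walks tile by tile through a Movement timeline, hopping on height changes.
; Rolled dice fill an action pool whose selected die gates actions, while hits drive anim states, dizziness and health-bar loss.
; Setters fire event dispatchers for state changes, and a picker widget resolves competing challengers.
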(event `self.ReceiveBeginPlay`
  (bind _shield_bar (`self.Shield Bar`))
  (`self.Set Character anim state` "NewEnumerator0")
  (bind _output_get (set `self.As WBP Health` (cast `/Game/Blueprints/HUD/Debug_Menu/WBP_Health` (`WidgetComponent.GetUserWidgetObject` (`self.HP Bar`)) :!pure true)))
  (`/Game/Blueprints/HUD/Debug_Menu/WBP_Health.Set Character` _output_get self)
  (bind _output_get_2 (set `self.As WBP Shield Bar` (cast `/Game/Blueprints/HUD/Debug_Menu/WBP_ShieldBar` (`WidgetComponent.GetUserWidgetObject` _shield_bar) :!pure true)))
  (`/Game/Blueprints/HUD/Debug_Menu/WBP_ShieldBar.Set Character` _output_get_2 self)
  (`SceneComponent.SetVisibility` _shield_bar false true))

(event `character Get's up`
  (`KismetSystemLibrary.Delay` 0.25)
  (`self.Set Character anim state` "NewEnumerator5")
  (`KismetSystemLibrary.Delay` 0.25)
  (`self.Set Character anim state` "NewEnumerator0"))

(event `Character Goes Dizzy`
  (bind _stats (break `/Game/Blueprints/Character/F_CharacterData` (`self.Character Data`)))
  (`KismetSystemLibrary.Delay` 2.0)
  (bind _structout (setmembers `/Game/Blueprints/Character/F_CharacterData_Stats` :`StructRef` _stats :`Number of Health Bars` (- (`.NumberofHealthBars_68_687FD87F4CC589428DED44B730C3BB0F` (break `/Game/Blueprints/Character/F_CharacterData_Stats` _stats)) 1)))
  (`self.Set Current Shield` (`.MaxHealth_62_1B087F1F4F92786D03E3848AF2433B7D` (break `/Game/Blueprints/Character/F_CharacterData_Stats` _structout)))
  (`self.Set Character anim state` "NewEnumerator5")
  (`/Game/Blueprints/HUD/Debug_Menu/WBP_Health.Update Health Bar` (`self.As WBP Health`)))

(event `Follow Path`
  (params (Path :type "Array of IntPoint Structure"))
  (if (> (`KismetArrayLibrary.Array_Length` Path) 0)
    (`self.On Character Started Walking` self)
    (set `self.Path` Path)
    (`self.ContinuetoFollow`)))

(event `ContinuetoFollow`
  (bind _movement (`self.Movement`))
  (bind _location (.location (`.TileTransform_9_C8B49F424080CB25DC8191A7EE85CF00` (break `/Game/Blueprints/Grid/F_TileData` (`BlueprintMapLibrary.Map_Find` (`/Game/Blueprints/Grid/BP_Grid.Grid Tiles Data` (`self.Grid`)) (`|GetArrayItem` (`self.Path`)))))))
  (bind (_returnvalue_roll _returnvalue_pitch _returnvalue_yaw) (`KismetMathLibrary.BreakRotator` (`KismetMathLibrary.FindLookAtRotation` (.location (`self.Previous Transform`)) _location)))
  (if (> (`KismetArrayLibrary.Array_Length` (`self.Path`)) 0)
    (`self.Set Character anim state` "NewEnumerator1")
    (set `self.Previous Transform` (`self.GetTransform`))
    (set `self.Next Transform` (`KismetMathLibrary.MakeTransform` _location (`KismetMathLibrary.MakeRotator` 0.0 0.0 _returnvalue_yaw)))
    (`TimelineComponent.SetPlayRate` _movement (/ (`TimelineComponent.GetTimelineLength` _movement) (`self.Move Duration per tile`)))
    (bind (_direction _location_alpha _roation_alpha _jump) (`Timeline|Movement` :!via `PlayFromStart`)
      (:`Update`
        (`self.K2_SetActorLocationAndRotation` (+ (`KismetMathLibrary.VLerp` (.location (`self.Previous Transform`)) (.location (`self.Next Transform`)) _location_alpha) (`KismetMathLibrary.MakeVector` 0.0 0.0 (`KismetMathLibrary.SelectFloat` 0.0 _jump (`KismetMathLibrary.NearlyEqual_FloatFloat` (.z (.location (`self.Next Transform`))) (.z (.location (`self.Previous Transform`))) 5.0)))) (`KismetMathLibrary.RLerp` (.rotation (`self.Previous Transform`)) (.rotation (`self.Next Transform`)) _roation_alpha true) false true))
      (:`Finished`
        (`self.Character Move anim end`)))
    (else
      (`self.Set Character anim state` "NewEnumerator0")
      (`self.On Character Finnished walking` self)
      (set `self.Moved This turn` true)
      (if (`.ReturnValue` (`BlueprintMapLibrary.Map_Find` (`.Tokens_73_F3A6EA8D45314AD8E266579E853C1E32` (break `/Game/Blueprints/Character/F_CharacterData_Stats` (`.Stats_8_5DCC378E48218015EE4248AF0BBAB223` (break `/Game/Blueprints/Character/F_CharacterData` (`self.Character Data`))))) "NewEnumerator4"))
        (`self.Modify Current Tokens` -1 "NewEnumerator4")))))

(fn `Activate Start of Turn Ability`)

(fn `Can do Action`
  (params (`Action data` :type "/Game/Blueprints/Core/Combat/Actions/Utility/F_ActionsData Structure"))
  (returns (`Can Cast` :type Boolean))
  (if (`KismetArrayLibrary.Array_Contains` (`.BasicActions_86_8C8A310B44A2D590338149A4969766A2` (break `/Game/Blueprints/Character/F_CharacterData_Stats` (`.Stats_8_5DCC378E48218015EE4248AF0BBAB223` (break `/Game/Blueprints/Character/F_CharacterData` (`self.Character Data`))))) (`.Action_5_B1DE74914B3203C13B02269484EF8DE6` (break `/Game/Blueprints/Core/Combat/Actions/Utility/F_ActionsData` `Action data`)))
    (if (>= (`self.Selected Die Number`) (`.Cost_17_A9E654AD403C5752B9FB40BEA2CFE651` (break `/Game/Blueprints/Core/Combat/Actions/Utility/F_ActionDataCast` (`.Cast_9_34DC641C48EEF71540EB4F8612D7E5A9` (break `/Game/Blueprints/Core/Combat/Actions/Utility/F_ActionsData` (`local.Action data`))))))
      (return true)
      (else
        (return false)))
    (else
      (return false))))

(fn `Character Hit By Action`
  (params (`Action Impact` :type "/Game/Blueprints/Core/Combat/Actions/Utility/F_ActionImpact Structure"))
  (locals (`Previous Health` :type Integer))
  (bind (_damagevalue _hpmodifier) (break `/Game/Blueprints/Core/Combat/Actions/Utility/F_ActionImpact` (`local.Action Impact`)))
  (set `local.Previous Health` (`.CurrentShield_66_A4511E234ADC7AEBA9BC4FB304200B85` (break `/Game/Blueprints/Character/F_CharacterData_Stats` (`.Stats_8_5DCC378E48218015EE4248AF0BBAB223` (break `/Game/Blueprints/Character/F_CharacterData` (`self.Character Data`))))))
  (if (!= _hpmodifier 0)
    (`self.Modify Character Health` _hpmodifier)
    (if (< (`.HPModifier_5_867480E44FB6616348E3D5BC16293E8D` (break `/Game/Blueprints/Core/Combat/Actions/Utility/F_ActionImpact` (`local.Action Impact`))) 0)
      (if (`self.Check is Health Bar Broken`)
        (`self.Set Character anim state` "NewEnumerator4")
        (if (not (`self.Check is Dead`))
          (`self.Character Goes Dizzy`))
        (else
          (`self.Set Character anim state` "NewEnumerator3")))
      (elif (== (`local.Previous Health`) 0)
        (`self.character Get's up`)))))

(fn `Character Move anim end`
  (locals (`Current Path Index` :type "IntPoint Structure"))
  (bind _grid (`self.Grid`))
  (bind _output_get (set `local.Current Path Index` (`.Index_10_EBED7CD648D9AC57BB540D8281F68B1E` (break `/Game/Blueprints/Grid/F_TileData` (`BlueprintMapLibrary.Map_Find` (`/Game/Blueprints/Grid/BP_Grid.Grid Tiles Data` _grid) (`|GetArrayItem` (`self.Path`)))))))
  (`/Game/Blueprints/Grid/BP_Grid.Remove State from Tile` _grid _output_get "NewEnumerator4")
  (`KismetArrayLibrary.Array_Remove` (`self.Path`))
  (`self.On Character Reach New Tile` self (`local.Current Path Index`)))

(fn `Check is Dead`
  (returns (`Is Dead` :type Boolean))
  (bind (_canmovediagonaly _validtiletypes _basicactions _currenthealth _maxhealth _currentshield _maxshield _numberofhealthbars) (break `/Game/Blueprints/Character/F_CharacterData_Stats` (`.Stats_8_5DCC378E48218015EE4248AF0BBAB223` (break `/Game/Blueprints/Character/F_CharacterData` (`self.Character Data`)))))
  (return (or (and (== _currenthealth 0) (== _numberofhealthbars 1)) (`self.Removed from play`))))

(fn `Check is Health Bar Broken`
  (returns (`Is Broken` :type Boolean))
  (return (== (`.CurrentHealth_61_D116B1B84C1D7A43AB51AD8484131249` (break `/Game/Blueprints/Character/F_CharacterData_Stats` (`.Stats_8_5DCC378E48218015EE4248AF0BBAB223` (break `/Game/Blueprints/Character/F_CharacterData` (`self.Character Data`))))) 0)))

(fn `Do Action`
  (params (`Target Index` :type "IntPoint Structure"))
  (`self.K2_SetActorRotation` (`KismetMathLibrary.FindLookAtRotation` (`KismetMathLibrary.MakeVector` (.x (`self.K2_GetActorLocation`)) (.y (`self.K2_GetActorLocation`))) (`KismetMathLibrary.MakeVector` (.x (.location (`.TileTransform_9_C8B49F424080CB25DC8191A7EE85CF00` (break `/Game/Blueprints/Grid/F_TileData` (`BlueprintMapLibrary.Map_Find` (`/Game/Blueprints/Grid/BP_Grid.Grid Tiles Data` (`self.Grid`)) `Target Index`))))) (.y (.location (`.TileTransform_9_C8B49F424080CB25DC8191A7EE85CF00` (break `/Game/Blueprints/Grid/F_TileData` (`BlueprintMapLibrary.Map_Find` (`/Game/Blueprints/Grid/BP_Grid.Grid Tiles Data` (`self.Grid`)) `Target Index`))))))))
  (`self.Set Character anim state` "NewEnumerator2"))

(fn `End Combat For Character`)

(fn `Get Unit Anim State`
  (returns (NewParam :type "/Game/Art/Characters/Enum_DebugAnimState Enum"))
  (return "NewEnumerator0"))

(fn `Modify Armor Value`
  (params (Value :type Integer))
  (bind _returnvalue (+ Value (`.Armor_92_9754266941D3B605E05576A2AC0B03ED` (break `/Game/Blueprints/Character/F_CharacterData_Stats` (`.Stats_8_5DCC378E48218015EE4248AF0BBAB223` (break `/Game/Blueprints/Character/F_CharacterData` (`self.Character Data`)))))))
  (if (< Value 0)
    (`self.Set Armor` true _returnvalue)
    (else
      (`self.Set Armor` false _returnvalue))))

(fn `Modify Character Action Pool`
  (params (`Is Add?` :type Boolean) (`Die Index` :type Integer) (`Die Number` :type Integer))
  (locals (`Action Pool` :type "Array of Integer"))
  (if (not (and (== `Die Index` -1) (== `Die Number` 0)))
    (set `local.Action Pool` (`.ActionPool_5_B5573866494C04EA2C02C882EFD84F22` (break `/Game/Blueprints/Character/F_CharacterData_Stance` (`self.Active Stance`))))
    (if (`local.Is Add?`)
      (`KismetArrayLibrary.Array_Add` (`local.Action Pool`) (`local.Die Number`))
      (else
        (`KismetArrayLibrary.Array_Remove` (`local.Action Pool`) (`local.Die Index`)))))
  (`self.Set Character Action Pool` (`local.Action Pool`)))

(fn `Modify Character Challanges`
  (params (`Is Challanger` :type Boolean) (`Target or Challanger` :type "/Game/Blueprints/Character/BP_Character Object Reference"))
  (bind _target_or_challanger (`local.Target or Challanger`))
  (if `Is Challanger`
    (`/Engine/EditorBlueprintResources/StandardMacros.IsValid` _target_or_challanger
      (:`Is Valid`
        (`KismetArrayLibrary.Array_Add` (`self.Challenged Characters`) _target_or_challanger)
        (`self.On Character Challenging` self)))
    (elif (or (== (`BlueprintMapLibrary.Map_Find` (`.Tokens_73_F3A6EA8D45314AD8E266579E853C1E32` (break `/Game/Blueprints/Character/F_CharacterData_Stats` (`.Stats_8_5DCC378E48218015EE4248AF0BBAB223` (break `/Game/Blueprints/Character/F_CharacterData` (`self.Character Data`))))) "NewEnumerator7") 0) (== (`self.Challenger`) (`local.Target or Challanger`)))
      (`self.Set Character Challenger` (`local.Target or Challanger`))
      (else
        (bind _returnvalue (`|CreateWidget` "/Game/Blueprints/HUD/Combat_Menu/WBP_ChallengerPicker.WBP_ChallengerPicker_C" (`GameplayStatics.GetPlayerController` 0) self (`self.Challenger`) (`local.Target or Challanger`)))
        (bind _output_get (set `self.Challenger Picker` _returnvalue))
        (`UserWidget.AddToPlayerScreen` _output_get 0)))))

(fn `Modify Character Health`
  (params (Modifier :type Integer))
  (`self.Set Current Health` (+ Modifier (`.CurrentHealth_61_D116B1B84C1D7A43AB51AD8484131249` (break `/Game/Blueprints/Character/F_CharacterData_Stats` (`.Stats_8_5DCC378E48218015EE4248AF0BBAB223` (break `/Game/Blueprints/Character/F_CharacterData` (`self.Character Data`)))))))
  (if (== (`local.Modifier`) 0)
    (`/Game/Blueprints/HUD/Debug_Menu/WBP_Health.Update Health Bar` (`self.As WBP Health`))
    (`|SpawnActorFromClass` "/Game/Blueprints/HUD/Debug_Menu/Utility/BP_AnimDamgaeNumbers.BP_AnimDamgaeNumbers_C" (`KismetMathLibrary.MakeTransform` (0.0 0.0 0.0)) "DontSpawnIfColliding" "MultiplyWithRoot" null (`local.Modifier`) null)))

(fn `Modify Character Shield`
  (params (Modifier :type Integer))
  (`self.Set Current Shield` (+ Modifier (`.CurrentShield_66_A4511E234ADC7AEBA9BC4FB304200B85` (break `/Game/Blueprints/Character/F_CharacterData_Stats` (`.Stats_8_5DCC378E48218015EE4248AF0BBAB223` (break `/Game/Blueprints/Character/F_CharacterData` (`self.Character Data`)))))))
  (if (== (`local.Modifier`) 0)
    (`/Game/Blueprints/HUD/Debug_Menu/WBP_ShieldBar.Update Shield Bar` (`self.As WBP Shield Bar`))
    (`|SpawnActorFromClass` "/Game/Blueprints/HUD/Debug_Menu/Utility/BP_AnimDamgaeNumbers.BP_AnimDamgaeNumbers_C" (`KismetMathLibrary.MakeTransform` (0.0 0.0 0.0)) "DontSpawnIfColliding" "MultiplyWithRoot" null (`local.Modifier`) null)))

(fn `Modify Current Tokens`
  (params (Value :type Integer) (Token :type "/Game/Blueprints/Character/Enum_Tokens Enum" :default "NewEnumerator0"))
  (bind (_value _returnvalue) (`BlueprintMapLibrary.Map_Find` (`.Tokens_73_F3A6EA8D45314AD8E266579E853C1E32` (break `/Game/Blueprints/Character/F_CharacterData_Stats` (`.Stats_8_5DCC378E48218015EE4248AF0BBAB223` (break `/Game/Blueprints/Character/F_CharacterData` (`self.Character Data`))))) (`local.Token`)))
  (if (`|EnumInequality` Token "NewEnumerator7")
    (if _returnvalue
      (`self.Set Current Tokens` (+ _value (`local.Value`)) (`local.Token`))
      (else
        (`self.Set Current Tokens` (`local.Value`) (`local.Token`))))))

(fn `Roll Action Dice`
  (`self.Set Action Pool From Dice` 1 1 1 1 1)
  (`self.Set Selected Number and Index` 0 -1))

(fn `Set Action Pool From Dice`
  (params (`Number of d4s` :type Integer) (`Number of d6s` :type Integer) (`Number of d8s` :type Integer) (`Number of d10s` :type Integer) (`Number of d12s` :type Integer))
  (for (_array_element _array_index) (`/Game/Blueprints/Core/Utility/BPFL_Utility.Roll Dice` `Number of d4s` `Number of d6s` `Number of d8s` `Number of d10s` `Number of d12s`)
    (`self.Modify Character Action Pool` true _array_index _array_element)))

(fn `Set Armor`
  (params (Triggered :type Boolean) (Value :type Integer))
  (locals (`Previous Armor` :type Integer))
  (bind _stats (break `/Game/Blueprints/Character/F_CharacterData` (`self.Character Data`)))
  (set `local.Previous Armor` (`.Armor_92_9754266941D3B605E05576A2AC0B03ED` (break `/Game/Blueprints/Character/F_CharacterData_Stats` _stats)))
  (bind _structout (setmembers `/Game/Blueprints/Character/F_CharacterData_Stats` :`StructRef` _stats :`Armor` Value))
  (setmembers `/Game/Blueprints/Character/F_CharacterData` :`StructRef` (`self.Character Data`) :`Stats` _structout)
  (if (`local.Triggered`)
    (set `local.Previous Armor` (select `bool` (== (`local.Value`) 0) :`false` (`KismetMathLibrary.Max` (- (`self.Armor Block Value`) 1) 1)))
    (`self.On Armor Triggered` self)
    (else
      (if (== (`local.Previous Armor`) 0)
        (set `local.Previous Armor` 3))
      (`self.On Character gain Armor` self))))

(fn `Set Character Action Pool`
  (params (`Action Pool` :type "Array of Integer"))
  (setmembers `/Game/Blueprints/Character/F_CharacterData_Stance` :`StructRef` (`self.Active Stance`) :`Action Pool` `Action Pool`)
  (`self.On Character Action Pool Change` self))

(fn `Set Character anim state`
  (params (`Anim State` :type "/Game/Art/Characters/Enum_DebugAnimState Enum" :default "NewEnumerator0"))
  (message `/Game/Art/Characters/BPI_UniAniations.Set Anim State` (`SkeletalMeshComponent.GetAnimInstance` (`self.Skeletal Mesh`)) `Anim State`))

(fn `Set Character Challenger`
  (params (Challenger :type "/Game/Blueprints/Character/BP_Character Object Reference"))
  (set `self.Challenger` Challenger)
  (`/Engine/EditorBlueprintResources/StandardMacros.IsValid` (`self.Challenger Picker`)
    (:`Is Valid`
      (`Widget.RemoveFromParent` (`self.Challenger Picker`))
      (set `self.Challenger Picker` null))
    (:`Is Not Valid`
      _))
  (`BlueprintMapLibrary.Map_Add` (`.Tokens_73_F3A6EA8D45314AD8E266579E853C1E32` (break `/Game/Blueprints/Character/F_CharacterData_Stats` (`.Stats_8_5DCC378E48218015EE4248AF0BBAB223` (break `/Game/Blueprints/Character/F_CharacterData` (`self.Character Data`))))) "NewEnumerator7" 1)
  (`KismetSystemLibrary.PrintString` "Challenged" true true (struct :`R` 1.0 :`B` 0.032419 :`A` 1.0))
  (`self.On Character Challenged` self))

(fn `Set Current Health`
  (params (Health :type Integer))
  (bind _structout (setmembers `/Game/Blueprints/Character/F_CharacterData_Stats` :`StructRef` (`.Stats_8_5DCC378E48218015EE4248AF0BBAB223` (break `/Game/Blueprints/Character/F_CharacterData` (`self.Character Data`))) :`Current Health` (`KismetMathLibrary.Clamp` Health 0 (`.MaxHealth_62_1B087F1F4F92786D03E3848AF2433B7D` (break `/Game/Blueprints/Character/F_CharacterData_Stats` (`.Stats_8_5DCC378E48218015EE4248AF0BBAB223` (break `/Game/Blueprints/Character/F_CharacterData` (`self.Character Data`))))))))
  (setmembers `/Game/Blueprints/Character/F_CharacterData` :`StructRef` (`self.Character Data`) :`Stats` _structout)
  (`self.On Character Health Change` self))

(fn `Set Current Shield`
  (params (Health :type Integer))
  (bind _structout (setmembers `/Game/Blueprints/Character/F_CharacterData_Stats` :`StructRef` (`.Stats_8_5DCC378E48218015EE4248AF0BBAB223` (break `/Game/Blueprints/Character/F_CharacterData` (`self.Character Data`))) :`Current Shield` (`KismetMathLibrary.Clamp` Health 0 (`.MaxShield_67_7805947F464FDC07BA60D19E5494BCB3` (break `/Game/Blueprints/Character/F_CharacterData_Stats` (`.Stats_8_5DCC378E48218015EE4248AF0BBAB223` (break `/Game/Blueprints/Character/F_CharacterData` (`self.Character Data`))))))))
  (setmembers `/Game/Blueprints/Character/F_CharacterData` :`StructRef` (`self.Character Data`) :`Stats` _structout)
  (`self.On Character Shield Change` self)
  (if (== (`.CurrentShield_66_A4511E234ADC7AEBA9BC4FB304200B85` (break `/Game/Blueprints/Character/F_CharacterData_Stats` (`.Stats_8_5DCC378E48218015EE4248AF0BBAB223` (break `/Game/Blueprints/Character/F_CharacterData` (`self.Character Data`))))) 0)
    (`SceneComponent.SetVisibility` (`self.Shield Bar`) false true)
    (else
      (`SceneComponent.SetVisibility` (`self.Shield Bar`) true true))))

(fn `Set Current Tokens`
  (params (`Modification Value` :type Integer) (Token :type "/Game/Blueprints/Character/Enum_Tokens Enum" :default "NewEnumerator0"))
  (locals (diffrence :type Integer))
  (bind (_canmovediagonaly _validtiletypes _basicactions _currenthealth _maxhealth _currentshield _maxshield _numberofhealthbars _tokens) (break `/Game/Blueprints/Character/F_CharacterData_Stats` (`.Stats_8_5DCC378E48218015EE4248AF0BBAB223` (break `/Game/Blueprints/Character/F_CharacterData` (`self.Character Data`)))))
  (bind _output_get (set `local.diffrence` (- (`local.Modification Value`) (`BlueprintMapLibrary.Map_Find` _tokens Token))))
  (if (!= _output_get 0)
    (`BlueprintMapLibrary.Map_Add` _tokens (`local.Token`) (`KismetMathLibrary.Clamp` (`local.Modification Value`) 0 10))
    (`self.On Character Token Change` self)))

(fn `Set Grid`
  (params (Grid :type "/Game/Blueprints/Grid/BP_Grid Object Reference"))
  (set `self.Grid` Grid))

(fn `Set Is Hovered`
  (params (`Is Hovered` :type Boolean))
  (set `self.Is Hovered` `Is Hovered`)
  (`self.On Hovered Character Change` self))

(fn `Set is Selected`
  (params (`Is Selected` :type Boolean))
  (set `self.Is Selected` `Is Selected`)
  (`self.On Selected Character Change` self))

(fn `Set Selected Number and Index`
  (params (`Selected Die Number` :type Integer) (`Selected Die Index` :type Integer))
  (set `self.Selected Die Number` `Selected Die Number`)
  (set `self.Selected Die Index` `Selected Die Index`)
  (`self.On Character Selected Number Change` self))

(fn `Set Team Index`
  (params (`Team Index` :type Integer))
  (bind _output_get (set `self.Team Index` `Team Index`))
  (bind _aswbp_health (cast `/Game/Blueprints/HUD/Debug_Menu/WBP_Health` (`WidgetComponent.GetWidget` (`self.HP Bar`))))
  (`ProgressBar.SetFillColorAndOpacity` (`/Game/Blueprints/HUD/Debug_Menu/WBP_Health.HealthBar` _aswbp_health) (`/Game/Blueprints/Core/Combat/Utility/BFL_Combat.Get Team Color` _output_get)))

(fn `Start Combat For Character`)

(fn `UserConstructionScript`
  (bind _skeletal_mesh (`self.Skeletal Mesh`))
  (bind (_canmovediagonaly _validtiletypes _basicactions _currenthealth _maxhealth _currentshield _maxshield _numberofhealthbars _tokens) (break `/Game/Blueprints/Character/F_CharacterData_Stats` (`.Stats_8_5DCC378E48218015EE4248AF0BBAB223` (break `/Game/Blueprints/Character/F_CharacterData` (`self.Character Data`)))))
  (`SkeletalMeshComponent.SetSkeletalMeshAsset` _skeletal_mesh "/Game/Art/Characters/Debug_Hero1/SK_Warrior.SK_Warrior")
  (`SkeletalMeshComponent.SetAnimInstanceClass` _skeletal_mesh "/Game/Art/Characters/Debug_Hero1/ABP_WarriorAnimation.ABP_WarriorAnimation_C")
  (`|ExecutionSequence`
    (:`then_0`
      (`BlueprintMapLibrary.Map_Add` _tokens "NewEnumerator0")
      (`BlueprintMapLibrary.Map_Add` _tokens "NewEnumerator1")
      (`BlueprintMapLibrary.Map_Add` _tokens "NewEnumerator2")
      (`BlueprintMapLibrary.Map_Add` _tokens "NewEnumerator3")
      (`BlueprintMapLibrary.Map_Add` _tokens "NewEnumerator4")
      (`BlueprintMapLibrary.Map_Add` _tokens "NewEnumerator6")
      (`BlueprintMapLibrary.Map_Add` _tokens "NewEnumerator7"))
    (:`then_1`
      (set `self.Active Stance` (make `/Game/Blueprints/Character/F_CharacterData_Stance` :`Range` (make `IntPoint` 1 1))))))