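; BP_GridModifier is an editor-visible grid tile marker that carries a tile type and shape and is hidden in game.
; Its construction script looks up the shape in DT_GridShapeData for mesh and material, then tints it translucently by tile type.
; It sets the first custom collision channel to Overlap, then immediately to Block, so it ends up blocking that channel.
; The event graph holds no logic.
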(fn `UserConstructionScript`
  (bind _staticmesh (`self.StaticMesh`))
  (bind _returnvalue (`|GetDataTableRow` "/Game/Blueprints/Grid/DT_GridShapeData.DT_GridShapeData" (`KismetStringLibrary.Conv_StringToName` (`|GetEnumeratorNameAsString` (`self.Tile Shape`))))
    (:`then`
      (bind (_meshsize _mesh _flatmesh _meshmaterial) (break `/Game/Blueprints/Grid/F_GridShapeData` _returnvalue))
      (`StaticMeshComponent.SetStaticMesh` _staticmesh _mesh)
      (`PrimitiveComponent.SetMaterial` _staticmesh 0 _meshmaterial)
      (`MeshComponent.SetVectorParameterValueOnMaterials` _staticmesh "Color" (`KismetMathLibrary.Conv_LinearColorToVector` (select `/Game/Blueprints/Grid/Modifiers/Enum_TileTypes` (`self.Tile Type`) :`NewEnumerator0` (struct :`A` 1.0) :`NewEnumerator1` (struct :`R` 0.536458 :`G` 0.122938 :`B` 0.138119 :`A` 1.0) :`NewEnumerator2` (struct :`R` 0.651042 :`A` 1.0) :`NewEnumerator6` (struct :`R` 0.817708 :`G` 0.817708 :`B` 0.817708 :`A` 1.0) :`NewEnumerator13` (struct :`G` 0.165606 :`B` 1.0 :`A` 1.0) :!type "LinearColor Structure")))
      (`MeshComponent.SetScalarParameterValueOnMaterials` _staticmesh "Opacity" 0.2)
      (`PrimitiveComponent.SetCollisionResponseToChannel` _staticmesh "ECC_GameTraceChannel1" "ECR_Overlap")
      (`PrimitiveComponent.SetCollisionResponseToChannel` _staticmesh "ECC_GameTraceChannel1" "ECR_Block")
      (`self.SetActorHiddenInGame` true))))