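; Grid tile renderer that draws tiles as instances of one Instanced Static Mesh, with mesh, material and collision set at initialization.
; A parallel index array maps tiles to instances, and adding a tile replaces its existing instance.
; Each instance receives color and fill opacity through custom data.
; Tactical mode colors by highest-priority obstacle, falling back to tile type; otherwise the highest-priority state sets a translucent highlight, or transparent without one.
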(fn `Add Instance`
  (params (InstanceTransform :type "Transform Structure (by ref)") (Index :type "IntPoint Structure (by ref)") (States :type "Array of /Game/Blueprints/Grid/Enum_TileStates Enum") (Obstacles :type "Array of /Game/Blueprints/Core/Combat/Obstacles/Utility/Enum_Obstacles Enum") (Type :type "/Game/Blueprints/Grid/Modifiers/Enum_TileTypes Enum" :default "NewEnumerator0"))
  (locals (NewLocalVar :type Integer :default 0))
  (bind _instancedstaticmesh (`self.InstancedStaticMesh`))
  (bind _i (`self.I`))
  (`self.RemoveInstaces` Index)
  (`InstancedStaticMeshComponent.AddInstance` (`self.InstancedStaticMesh`) InstanceTransform false)
  (bind _returnvalue (`KismetArrayLibrary.Array_Add` (`self.Instace Indexs`) Index))
  (set `self.I` _returnvalue)
  (bind (_color _fill_opacity) (`self.Get Color Of Tile` States Obstacles Type))
  (bind (_r _g _b) (`KismetMathLibrary.BreakColor` _color))
  (`InstancedStaticMeshComponent.SetCustomDataValue` _instancedstaticmesh _i 0 _r false)
  (`InstancedStaticMeshComponent.SetCustomDataValue` _instancedstaticmesh _i 1 _g false)
  (`InstancedStaticMeshComponent.SetCustomDataValue` _instancedstaticmesh _i 2 _b false)
  (`InstancedStaticMeshComponent.SetCustomDataValue` _instancedstaticmesh _i 3 _fill_opacity false))

(fn `ClearInst`
  (`InstancedStaticMeshComponent.ClearInstances` (`self.InstancedStaticMesh`))
  (`KismetArrayLibrary.Array_Clear` (`self.Instace Indexs`)))

(fn `Get Color Of Tile`
  (params (States :type "Array of /Game/Blueprints/Grid/Enum_TileStates Enum") (Obstacles :type "Array of /Game/Blueprints/Core/Combat/Obstacles/Utility/Enum_Obstacles Enum") (Type :type "/Game/Blueprints/Grid/Modifiers/Enum_TileTypes Enum" :default "NewEnumerator0"))
  (returns (color :type "LinearColor Structure") (`Fill Opacity` :type "Float (double-precision)"))
  (if (`self.Generate Tactical`)
    (if (== (`KismetArrayLibrary.Array_Length` (`local.Obstacles`)) 0)
      (return (select `/Game/Blueprints/Grid/Modifiers/Enum_TileTypes` (`local.Type`) :`NewEnumerator0` (struct :`G` 0.445201 :`B` 0.005605 :`A` 1.0) :`NewEnumerator2` (struct :`G` 0.445201 :`B` 0.005605 :`A` 1.0) :`NewEnumerator6` (struct :`R` 1.0 :`B` 0.544227 :`A` 1.0) :`NewEnumerator13` (struct :`G` 0.115468 :`B` 0.445201 :`A` 1.0) :!type "LinearColor Structure") 1.0)
      (else
        (for _array_element (`|MakeArray` "NewEnumerator9" "NewEnumerator13" "NewEnumerator11" "NewEnumerator12" "NewEnumerator8" "NewEnumerator7" :!type "/Game/Blueprints/Core/Combat/Obstacles/Utility/Enum_Obstacles Enum")
          (if (`KismetArrayLibrary.Array_Contains` (`local.Obstacles`) _array_element)
            (return (select `/Game/Blueprints/Core/Combat/Obstacles/Utility/Enum_Obstacles` _array_element :`NewEnumerator6` (struct :`G` 0.445201 :`B` 0.005605 :`A` 1.0) :`NewEnumerator7` (struct :`R` 0.174108 :`B` 0.359375 :`A` 1.0) :`NewEnumerator8` (struct :`R` 1.0 :`G` 0.633058 :`A` 1.0) :`NewEnumerator9` (struct :`G` 0.234551 :`B` 1.0 :`A` 1.0) :`NewEnumerator10` (struct :`G` 0.445201 :`B` 0.005605 :`A` 1.0) :`NewEnumerator11` (struct :`R` 0.302083 :`A` 1.0) :`NewEnumerator12` (struct :`R` 0.109375 :`G` 0.109375 :`B` 0.109375 :`A` 1.0) :`NewEnumerator13` (struct :`G` 0.234551 :`B` 1.0 :`A` 1.0) :!type "LinearColor Structure") 1.0)))
        (return (select `/Game/Blueprints/Grid/Modifiers/Enum_TileTypes` (`local.Type`) :`NewEnumerator0` (struct :`G` 0.445201 :`B` 0.005605 :`A` 1.0) :`NewEnumerator2` (struct :`G` 0.445201 :`B` 0.005605 :`A` 1.0) :`NewEnumerator6` (struct :`R` 1.0 :`B` 0.544227 :`A` 1.0) :`NewEnumerator13` (struct :`G` 0.115468 :`B` 0.445201 :`A` 1.0) :!type "LinearColor Structure") 1.0)))
    (elif (== (`KismetArrayLibrary.Array_Length` States) 0)
      (return (struct :`A` 1.0) 0.0)
      (else
        (for _array_element_2 (`|MakeArray` "NewEnumerator7" "NewEnumerator8" "NewEnumerator6" "NewEnumerator5" "NewEnumerator2" "NewEnumerator1" "NewEnumerator4" "NewEnumerator3" :!type "/Game/Blueprints/Grid/Enum_TileStates Enum")
          (if (`KismetArrayLibrary.Array_Contains` (`local.States`) _array_element_2)
            (return (select `/Game/Blueprints/Grid/Enum_TileStates` _array_element_2 :`NewEnumerator0` (struct :`A` 1.0) :`NewEnumerator1` (struct :`R` 0.890983 :`G` 1.0 :`A` 1.0) :`NewEnumerator2` (struct :`R` 0.065589 :`G` 1.0 :`A` 1.0) :`NewEnumerator3` (struct :`G` 0.475082 :`B` 0.479167 :`A` 1.0) :`NewEnumerator4` (struct :`R` 0.399372 :`B` 1.0 :`A` 1.0) :`NewEnumerator5` (struct :`R` 0.59375 :`B` 0.143655 :`A` 1.0) :`NewEnumerator6` (struct :`G` 0.340517 :`B` 0.927083 :`A` 1.0) :`NewEnumerator7` (struct :`R` 1.0 :`G` 0.89028 :`B` 0.541667 :`A` 1.0) :`NewEnumerator8` (struct :`R` 0.364583 :`B` 0.003626 :`A` 1.0) :!type "LinearColor Structure") 0.2)))
        (return (struct :`A` 1.0) 0.0)))))

(fn `InitializeGridInst`
  (params (Mesh :type "StaticMesh Object Reference") (Material :type "MaterialInterface Object Reference") (Collision :type "ECollisionEnabled Enum" :default "NoCollision") (`Generate for Types` :type Boolean))
  (bind _instancedstaticmesh (`self.InstancedStaticMesh`))
  (`StaticMeshComponent.SetStaticMesh` _instancedstaticmesh Mesh)
  (`PrimitiveComponent.SetMaterial` _instancedstaticmesh 0 Material)
  (set `self.Generate Tactical` `Generate for Types`)
  (`PrimitiveComponent.SetCollisionEnabled` _instancedstaticmesh Collision))

(fn `RemoveInstaces`
  (params (Index :type "IntPoint Structure (by ref)"))
  (bind _instace_indexs (`self.Instace Indexs`))
  (if (`KismetArrayLibrary.Array_Contains` _instace_indexs Index)
    (`InstancedStaticMeshComponent.RemoveInstance` (`self.InstancedStaticMesh`) (`KismetArrayLibrary.Array_Find` _instace_indexs Index))
    (`KismetArrayLibrary.Array_RemoveItem` _instace_indexs Index)))

(fn `UserConstructionScript`)