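; Debug actor that draws text over walkable grid tiles showing their index, pathfinding costs and discovery sort order.
; After a short delay on BeginPlay, it finds BP_Grid and binds to grid and pathfinding update and clear delegates.
; ShowTileText sets the display toggles, then refreshes every tile or clears all text.
; UpdateTextOnTile builds each label, using TextRenderActors spawned on demand and cached in a map by tile index.
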(event `self.ReceiveBeginPlay`
  (bind _as_bp_pathfinding (`/Game/Blueprints/Grid/BP_Grid.As BP Pathfinding` (`self.Grid`)))
  (`KismetSystemLibrary.Delay` 0.2)
  (bind _returnvalue (`GameplayStatics.GetActorOfClass` "/Game/Blueprints/Grid/BP_Grid.BP_Grid_C"))
  (bind _output_get (set `self.Grid` _returnvalue))
  (add `/Game/Blueprints/Grid/BP_Grid.OnTileDataUpdated` _output_get (`|CreateDelegate` :!event `Update text on Tile`))
  (add `/Game/Blueprints/Grid/BP_Grid.On Grid Destroyed` _output_get (`|CreateDelegate` :!event `Clear All Text Actors`))
  (add `/Game/Blueprints/Character/BP_Pathfinding.On Pathfinding Data Updated` _as_bp_pathfinding (`|CreateDelegate` :!event `Update text on Tile`))
  (add `/Game/Blueprints/Character/BP_Pathfinding.On Pathfinding Data Cleared` _as_bp_pathfinding (`|CreateDelegate` :!event `Clear All Text Actors`)))

(event `ReupdateText_Event`
  (params (Index :type "IntPoint Structure"))
  (`KismetSystemLibrary.RetriggerableDelay` 0.1)
  (`self.Update text on Tile` Index))

(fn `Clear All Text Actors`
  (bind _values (`BlueprintMapLibrary.Map_Values` (`self.Spawn Text`)))
  (for _array_element _values
    (`self.K2_DestroyActor` _array_element))
  (`BlueprintMapLibrary.Map_Clear` (`self.Spawn Text`)))

(fn `Destroy Text Actor`
  (params (Index :type "IntPoint Structure"))
  (locals (Actor :type "TextRenderActor Object Reference"))
  (bind _output_get (set `local.Actor` (`BlueprintMapLibrary.Map_Find` (`self.Spawn Text`) Index)))
  (`/Engine/EditorBlueprintResources/StandardMacros.IsValid` _output_get
    (:`Is Valid`
      (`self.K2_DestroyActor` _output_get)
      (`BlueprintMapLibrary.Map_Remove` (`self.Spawn Text`) (`local.Index`)))))

(fn `Get Text Actor`
  (params (Index :type "IntPoint Structure"))
  (returns (`Text Actor` :type "TextRenderActor Object Reference"))
  (locals (Actor :type "TextRenderActor Object Reference"))
  (bind _actor (`local.Actor`))
  (bind _textrender (`TextRenderActor.TextRender` _actor))
  (bind _output_get (set `local.Actor` (`BlueprintMapLibrary.Map_Find` (`self.Spawn Text`) Index)))
  (`/Engine/EditorBlueprintResources/StandardMacros.IsValid` _output_get
    (:`Is Valid`
      (return _output_get))
    (:`Is Not Valid`
      (bind _returnvalue (`|SpawnActorFromClass` "/Script/Engine.TextRenderActor" (`KismetMathLibrary.MakeTransform` (0.0 0.0 0.0)) "AlwaysSpawn" "MultiplyWithRoot" null null))
      (bind _output_get_2 (set `local.Actor` _returnvalue))
      (`BlueprintMapLibrary.Map_Add` (`self.Spawn Text`) (`local.Index`) _output_get_2)
      (`self.SetActorTickEnabled` _actor false)
      (`self.SetActorEnableCollision` _actor false)
      (`TextRenderComponent.SetHorizontalAlignment` _textrender "EHTA_Center")
      (`TextRenderComponent.SetVerticalAlignment` _textrender "EVRTA_TextCenter")
      (return (`local.Actor`)))))

(fn `Show Tile Text`
  (params (`P_Show Indexes` :type Boolean) (`P_Show Cost to Enter` :type Boolean) (`P_Show Cost to Target` :type Boolean) (`P_Show Cost From Start` :type Boolean) (`P_Show Sort Order` :type Boolean))
  (`|ExecutionSequence`
    (:`then_0`
      (set `self.Show Indexes` (`local.P_Show Indexes`))
      (set `self.Show Cost to Enter` (`local.P_Show Cost to Enter`))
      (set `self.Show Cost to Target` (`local.P_Show Cost to Target`))
      (set `self.Show Sort Order` (`local.P_Show Sort Order`))
      (set `self.Show Cost From Start` (`local.P_Show Cost From Start`)))
    (:`then_1`
      (if (or (`local.P_Show Indexes`) (`local.P_Show Cost to Enter`) (`local.P_Show Cost to Target`) (`local.P_Show Cost From Start`) (`local.P_Show Sort Order`))
        (bind _keys (`BlueprintMapLibrary.Map_Keys` (`/Game/Blueprints/Grid/BP_Grid.Grid Tiles Data` (`self.Grid`))))
        (for _array_element _keys
          (`self.Update text on Tile` _array_element))
        (else
          (`self.Clear All Text Actors`))))))

(fn `Update text on Tile`
  (params (Index :type "IntPoint Structure"))
  (locals (Data :type "/Game/Blueprints/Grid/F_TileData Structure") (`Text Actor` :type "TextRenderActor Object Reference") (Text :type "Array of String") (`Pathfinding Data` :type "/Game/Blueprints/Grid/F_PathfindingData Structure") (`Text Length` :type "Array of Integer") (NewLocalVar :type "Transform Structure"))
  (bind (_index_x _index_y) (break `IntPoint` (`local.Index`)))
  (bind (_index _previousindex _costtoentertile _costfromthestart _minimalcosttotarget) (break `/Game/Blueprints/Grid/F_PathfindingData` (`local.Pathfinding Data`)))
  (bind (_index_2 _previousindex_2 _costtoentertile_2 _costfromthestart_2) (break `/Game/Blueprints/Grid/F_PathfindingData` (`local.Pathfinding Data`)))
  (bind _as_bp_pathfinding (`/Game/Blueprints/Grid/BP_Grid.As BP Pathfinding` (`self.Grid`)))
  (bind (_tile_size_x _tile_size_y) (`KismetMathLibrary.BreakVector` (`/Game/Blueprints/Grid/BP_Grid.Tile Size` (`self.Grid`))))
  (bind (_value _returnvalue) (`BlueprintMapLibrary.Map_Find` (`/Game/Blueprints/Grid/BP_Grid.Grid Tiles Data` (`self.Grid`)) (`local.Index`)))
  (bind _returnvalue_2 (`KismetArrayLibrary.Array_Find` (`/Game/Blueprints/Character/BP_Pathfinding.Discovered Tiles` _as_bp_pathfinding) (`local.Index`)))
  (bind (_value_2 _returnvalue_3) (`BlueprintMapLibrary.Map_Find` (`/Game/Blueprints/Character/BP_Pathfinding.Pathfinding Data` (`/Game/Blueprints/Grid/BP_Grid.As BP Pathfinding` (`self.Grid`))) (`local.Index`)))
  (bind _returnvalue_4 (`KismetStringLibrary.Concat_StrStr` "Enter: " (`KismetStringLibrary.Conv_IntToString` (`.CostToEnterTile_10_CD261BB54EAC367A21D2509DC1B718BB` (break `/Game/Blueprints/Grid/F_PathfindingData` (`local.Pathfinding Data`))))))
  (bind _returnvalue_5 (`KismetStringLibrary.Concat_StrStr` "Min: " (`KismetStringLibrary.Conv_IntToString` _minimalcosttotarget)))
  (bind _returnvalue_6 (`KismetStringLibrary.Concat_StrStr` "Start: " (`KismetStringLibrary.Conv_IntToString` _costfromthestart_2)))
  (bind _returnvalue_7 (`KismetStringLibrary.Concat_StrStr` "Sort: " (`KismetStringLibrary.Conv_IntToString` _returnvalue_2) "[" (`KismetStringLibrary.Conv_IntToString` (`|GetArrayItem` (`/Game/Blueprints/Character/BP_Pathfinding.Discovered Tile Sorting Cost` _as_bp_pathfinding) _returnvalue_2)) "]"))
  (if (or (`self.Show Indexes`) (`self.Show Cost to Enter`) (`self.Show Cost to Target`) (`self.Show Cost From Start`) (`self.Show Sort Order`))
    (if _returnvalue
      (bind _output_get (set `local.Data` _value))
      (if (`/Game/Blueprints/Core/Utility/BPFL_Utility.Is Tile Type Walkable` (`.TileType_7_99A5401643D0FD504FC2D2B4806678DB` (break `/Game/Blueprints/Grid/F_TileData` _output_get)))
        (`|ExecutionSequence`
          (:`then_0`
            (if (`self.Show Indexes`)
              (`KismetArrayLibrary.Array_Add` (`local.Text`) (`KismetStringLibrary.Concat_StrStr` "(" (`KismetStringLibrary.Conv_IntToString` _index_x) "," (`KismetStringLibrary.Conv_IntToString` _index_y) ")"))))
          (:`then_1`
            (if (or (`self.Show Cost to Enter`) (`self.Show Cost to Target`) (`self.Show Cost From Start`) (`self.Show Sort Order`))
              (if _returnvalue_3
                (set `local.Pathfinding Data` _value_2)
                (`|ExecutionSequence`
                  (:`then_0`
                    (if (`self.Show Cost to Enter`)
                      (`KismetArrayLibrary.Array_Add` (`local.Text`) _returnvalue_4)
                      (`KismetArrayLibrary.Array_Add` (`local.Text Length`) (`KismetStringLibrary.Len` _returnvalue_4))))
                  (:`then_1`
                    (if (`self.Show Cost to Target`)
                      (if (!= _minimalcosttotarget 99999)
                        (`KismetArrayLibrary.Array_Add` (`local.Text`) _returnvalue_5)
                        (`KismetArrayLibrary.Array_Add` (`local.Text Length`) (`KismetStringLibrary.Len` _returnvalue_5)))))
                  (:`then_2`
                    (if (`self.Show Cost From Start`)
                      (if (!= _costfromthestart_2 99999)
                        (`KismetArrayLibrary.Array_Add` (`local.Text`) _returnvalue_6)
                        (`KismetArrayLibrary.Array_Add` (`local.Text Length`) (`KismetStringLibrary.Len` _returnvalue_6)))))
                  (:`then_3`
                    (if (`self.Show Sort Order`)
                      (if (!= _returnvalue_2 -1)
                        (`KismetArrayLibrary.Array_Add` (`local.Text`) _returnvalue_7)
                        (`KismetArrayLibrary.Array_Add` (`local.Text Length`) (`KismetStringLibrary.Len` _returnvalue_7)))))))))
          (:`then_2`
            (if (> (`KismetArrayLibrary.Array_Length` (`local.Text`)) 0)
              (bind _text_actor (`self.Get Text Actor` (`local.Index`)))
              (set `local.Text Actor` _text_actor)
              (`TextRenderComponent.K2_SetText` (`TextRenderActor.TextRender` (`local.Text Actor`)) (`KismetTextLibrary.Conv_StringToText` (`KismetStringLibrary.JoinStringArray` (`local.Text`) " \n")))
              (`self.K2_SetActorTransform` (`local.Text Actor`) (`KismetMathLibrary.MakeTransform` (+ (.location (`.TileTransform_9_C8B49F424080CB25DC8191A7EE85CF00` (break `/Game/Blueprints/Grid/F_TileData` (`local.Data`)))) (0.0 0.0 2.0)) (struct :`Pitch` 90.0 :`Yaw` 180.0) (`KismetMathLibrary.Conv_DoubleToVector` (/ _tile_size_y 100.0))) false false)
              (else
                (`self.Destroy Text Actor` (`local.Index`))))))))))

(fn `UserConstructionScript`)