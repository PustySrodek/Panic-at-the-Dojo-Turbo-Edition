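; BP_GridVisual renders the grid's tiles through two BP_GridMeshInst child actors: a flat bordered grid and a toggleable tactical grid.
; Tile updates remove and re-add instances by index, with the flat layer showing only walkable tiles at a configurable ground offset.
; Tactical mode hides "NT"-tagged actors and enables tactical collision.
; Tactical updates made while the mode is off are deferred to a full rebuild on next enable.
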(fn `Destroy Grid Visual`
  (bind _as_grid_mesh_inst (`self.As Grid Mesh Inst`))
  (bind _as_tactical_mesh_inst_0 (`self.As Tactical Mesh Inst_0`))
  (`/Engine/EditorBlueprintResources/StandardMacros.IsValid` _as_grid_mesh_inst
    (:`Is Valid`
      (`/Game/Blueprints/Grid/BP_GridMeshInst.ClearInst` _as_grid_mesh_inst)
      (`/Engine/EditorBlueprintResources/StandardMacros.IsValid` _as_tactical_mesh_inst_0
        (:`Is Valid`
          (`/Game/Blueprints/Grid/BP_GridMeshInst.ClearInst` _as_tactical_mesh_inst_0))))))

(fn `Initialize Grid Visual`
  (params (Grid :type "/Game/Blueprints/Grid/BP_Grid Object Reference"))
  (bind (_meshsize _mesh _flatmesh _meshmaterial _bordermeshmaterial _tacticalmeshmaterial) (break `/Game/Blueprints/Grid/F_GridShapeData` (`/Game/Blueprints/Grid/BP_Grid.Out Row` (`self.Grid`))))
  (bind (_meshsize_2 _mesh_2 _flatmesh_2 _meshmaterial_2 _bordermeshmaterial_2) (break `/Game/Blueprints/Grid/F_GridShapeData` (`/Game/Blueprints/Grid/BP_Grid.Out Row` (`self.Grid`))))
  (set `self.Grid` Grid)
  (set `self.As Grid Mesh Inst` (cast `/Game/Blueprints/Grid/BP_GridMeshInst` (`ChildActorComponent.ChildActor` (`self.Grid Mesh Inst`)) :!pure true))
  (set `self.As Tactical Mesh Inst_0` (cast `/Game/Blueprints/Grid/BP_GridMeshInst` (`ChildActorComponent.ChildActor` (`self.Tactical Grid Mesh Inst`)) :!pure true))
  (`/Game/Blueprints/Grid/BP_GridMeshInst.InitializeGridInst` (`self.As Grid Mesh Inst`) _flatmesh_2 _bordermeshmaterial_2 "QueryOnly" false)
  (`/Game/Blueprints/Grid/BP_GridMeshInst.InitializeGridInst` (`self.As Tactical Mesh Inst_0`) _mesh _tacticalmeshmaterial "QueryOnly" true)
  (`self.K2_SetActorLocation` (0.0 0.0 0.0))
  (`self.Set Offset from Ground` (`self.Offset`))
  (`self.Set Is Tactical` (`self.Is Grid Tactical`)))

(fn `Set Is Tactical`
  (params (`Tactical Grid` :type Boolean))
  (bind _as_tactical_mesh_inst_0 (`self.As Tactical Mesh Inst_0`))
  (bind _grid (`self.Grid`))
  (bind _output_get (set `self.Is Grid Tactical` `Tactical Grid`))
  (`SceneComponent.SetHiddenInGame` (`self.Tactical Grid Mesh Inst`) (not _output_get) false)
  (bind _outactors (`GameplayStatics.GetAllActorsWithTag` "NT"))
  (for _array_element _outactors
    (`self.SetActorHiddenInGame` _array_element (`self.Is Grid Tactical`)))
  (`|ExecutionSequence`
    (:`then_0`
      (if (and (`self.Is Grid Tactical`) (`self.ReGen Tactical on next enable`))
        (set `self.ReGen Tactical on next enable` false)
        (`/Engine/EditorBlueprintResources/StandardMacros.IsValid` _grid
          (:`Is Valid`
            (bind _values (`BlueprintMapLibrary.Map_Values` (`/Game/Blueprints/Grid/BP_Grid.Grid Tiles Data` _grid)))
            (for _array_element_2 _values
              (`self.Update Tile Visual` _array_element_2))))))
    (:`then_1`
      (`/Engine/EditorBlueprintResources/StandardMacros.IsValid` _as_tactical_mesh_inst_0
        (:`Is Valid`
          (`PrimitiveComponent.SetCollisionEnabled` (`/Game/Blueprints/Grid/BP_GridMeshInst.InstancedStaticMesh` _as_tactical_mesh_inst_0) (select `bool` (`self.Is Grid Tactical`) :`false` "NoCollision" :`true` "QueryOnly" :!type "ECollisionEnabled Enum")))))))

(fn `Set Offset from Ground`
  (params (Offset :type "Float (double-precision)"))
  (bind _output_get (set `self.Offset` Offset))
  (`SceneComponent.K2_SetRelativeLocation` (`self.Grid Mesh Inst`) (`KismetMathLibrary.MakeVector` 0.0 0.0 _output_get) false false))

(fn `Update Tactical Visual`
  (params (Data :type "/Game/Blueprints/Grid/F_TileData Structure"))
  (bind (_data_index _data_tiletype _data_tiletransform _data_tilestate) (break `/Game/Blueprints/Grid/F_TileData` (`local.Data`)))
  (bind (_data_index_2 _data_tiletype_2) (break `/Game/Blueprints/Grid/F_TileData` (`local.Data`)))
  (bind _as_tactical_mesh_inst_0 (`self.As Tactical Mesh Inst_0`))
  (if (`self.Is Grid Tactical`)
    (`/Game/Blueprints/Grid/BP_GridMeshInst.RemoveInstaces` _as_tactical_mesh_inst_0 _data_index_2)
    (if (`|EnumInequality` _data_tiletype_2 "NewEnumerator1")
      (`/Game/Blueprints/Grid/BP_GridMeshInst.Add Instance` _as_tactical_mesh_inst_0 _data_tiletransform _data_index _data_tilestate _data_tiletype))
    (else
      (set `self.ReGen Tactical on next enable` true))))

(fn `Update Tile Visual`
  (params (Data :type "/Game/Blueprints/Grid/F_TileData Structure"))
  (bind _as_grid_mesh_inst (`self.As Grid Mesh Inst`))
  (bind (_data_index _data_tiletype _data_tiletransform _data_tilestate) (break `/Game/Blueprints/Grid/F_TileData` (`local.Data`)))
  (`|ExecutionSequence`
    (:`then_0`
      (`/Game/Blueprints/Grid/BP_GridMeshInst.RemoveInstaces` _as_grid_mesh_inst _data_index)
      (if (`/Game/Blueprints/Core/Utility/BPFL_Utility.Is Tile Type Walkable` _data_tiletype)
        (`/Game/Blueprints/Grid/BP_GridMeshInst.Add Instance` _as_grid_mesh_inst _data_tiletransform _data_index _data_tilestate _data_tiletype)))
    (:`then_1`
      (`self.Update Tactical Visual` Data))))

(fn `UserConstructionScript`)