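; BP_Grid is the tile grid actor that builds and stores square or hex tiles, with walkability, state and obstacle queries.
; Its construction script links child visual and pathfinding actors, then spawns tiles from shape table data, optionally sphere-tracing for ground height and BP_GridModifier types.
; Hex tiles use doubled-Y indexing, and cursor traces convert to tile indices.
; Tile edits update the visual and fire events, with a state-to-index map for lookups.
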(event `self.ReceiveBeginPlay`
  (set `self.Tile Count` (make `IntPoint` 15 15))
  (set `self.Tile Size` (`self.Get Tile Size from Grid Shape` (`self.Tile Shape`))))

(fn `Add Grid Tile`
  (params (Data :type "/Game/Blueprints/Grid/F_TileData Structure"))
  (locals (`Tile Data` :type "/Game/Blueprints/Grid/F_TileData Structure"))
  (bind (_index _tiletype _tiletransform) (break `/Game/Blueprints/Grid/F_TileData` (`local.Tile Data`)))
  (bind _output_get (set `local.Tile Data` Data))
  (`BlueprintMapLibrary.Map_Add` (`self.Grid Tiles Data`) (`.Index_10_EBED7CD648D9AC57BB540D8281F68B1E` (break `/Game/Blueprints/Grid/F_TileData` _output_get)) _output_get)
  (`/Game/Blueprints/Grid/BP_GridVisual.Update Tile Visual` (`self.As BP Grid Visual`) (make `/Game/Blueprints/Grid/F_TileData` _index _tiletype _tiletransform _ null))
  (`self.OnTileDataUpdated` (`.Index_10_EBED7CD648D9AC57BB540D8281F68B1E` (break `/Game/Blueprints/Grid/F_TileData` (`local.Tile Data`)))))

(fn `Add State to Tile`
  (params (Index :type "IntPoint Structure") (State :type "/Game/Blueprints/Grid/Enum_TileStates Enum" :default "NewEnumerator0"))
  (locals (Data :type "/Game/Blueprints/Grid/F_TileData Structure"))
  (bind _data_index (break `/Game/Blueprints/Grid/F_TileData` (`local.Data`)))
  (bind (_value _returnvalue) (`BlueprintMapLibrary.Map_Find` (`self.Grid Tiles Data`) Index))
  (if _returnvalue
    (bind _output_get (set `local.Data` _value))
    (bind _returnvalue_2 (`KismetArrayLibrary.Array_AddUnique` (`.TileState_15_2CD077A14CF44985E0DDB1AF1B2DA5B7` (break `/Game/Blueprints/Grid/F_TileData` _output_get)) State))
    (if (>= _returnvalue_2 0)
      (`BlueprintMapLibrary.Map_Add` (`self.Grid Tiles Data`) _data_index (`local.Data`))
      (bind _indexe (`self.Get All Tiles With State` (`local.State`)))
      (`KismetArrayLibrary.Array_Add` _indexe (`local.Index`))
      (`BlueprintMapLibrary.Map_Add` (`self.Tile State To Indexes`) (`local.State`) (make `/Game/Blueprints/Grid/F_IntPointArray` _indexe))
      (`/Game/Blueprints/Grid/BP_GridVisual.Update Tile Visual` (`self.As BP Grid Visual`) (`local.Data`))
      (`self.On Tile State Updated` (`local.Index`)))))

(fn `Calculate Origin Point`
  (returns (Origin :type "Vector Structure") (Center :type "Vector Structure"))
  (locals (C :type "Vector Structure" :default (0.0 0.0 0.0)))
  (bind (_tile_count_x _tile_count_y) (break `IntPoint` (`self.Tile Count`)))
  (bind _v_final (`/Game/Blueprints/Core/Utility/BPFL_Utility.Snap Vector to Vector` (`self.Center Location`) (`self.Tile Size`)))
  (bind (_returnvalue_x _returnvalue_y) (break `IntPoint` (/ (- (`self.Tile Count`) (select `bool` (`/Game/Blueprints/Core/Utility/BPFL_Utility.Is Int Even` _tile_count_x) :`false` (make `IntPoint` 0) :`true` (make `IntPoint` 1 1) :!type "IntPoint Structure") (select `bool` (`/Game/Blueprints/Core/Utility/BPFL_Utility.Is Int Even` _tile_count_y) :`false` (make `IntPoint` 0) :`true` (make `IntPoint` 1 1) :!type "IntPoint Structure")) (make `IntPoint` 2 2))))
  (switch `/Game/Blueprints/Grid/Enum_GridShapeData` (`self.Tile Shape`)
    (:`NewEnumerator1`
      (return (- _v_final (* (`KismetMathLibrary.MakeVector` (`KismetMathLibrary.Conv_IntToDouble` _returnvalue_x) (`KismetMathLibrary.Conv_IntToDouble` _returnvalue_y)) (`self.Tile Size`))) _v_final))
    (:`NewEnumerator2`
      (set `local.C` (`/Game/Blueprints/Core/Utility/BPFL_Utility.Snap Vector to Vector` (`self.Center Location`) (* (`self.Tile Size`) (2.0 1.0 1.0))))
      (return (- (`local.C`) (`/Game/Blueprints/Core/Utility/BPFL_Utility.Snap Vector to Vector` (* (`KismetMathLibrary.Conv_IntPointToVector2D` (/ (`self.Tile Count`) (make `IntPoint` 3 2))) (`self.Tile Size`)) (* (`self.Tile Size`) (1.5 1.0 1.0)))) (`local.C`)))))

(fn `Clear All States from Tiles`
  (params (State :type "/Game/Blueprints/Grid/Enum_TileStates Enum" :default "NewEnumerator0"))
  (bind _indexe (`self.Get All Tiles With State` State))
  (for _array_element _indexe
    (`self.Remove State from Tile` _array_element State)))

(fn `Destroy Grid`
  (`BlueprintMapLibrary.Map_Clear` (`self.Grid Tiles Data`))
  (`/Game/Blueprints/Grid/BP_GridVisual.Destroy Grid Visual` (`self.As BP Grid Visual`))
  (`self.On Grid Destroyed`))

(fn `Get all Tiles with Obstacle`
  (params (Obstacle :type "/Game/Blueprints/Core/Combat/Obstacles/Utility/Enum_Obstacles Enum" :default "NewEnumerator6"))
  (returns (Indexes :type "Array of IntPoint Structure"))
  (locals (`Obstacle Indexes` :type "Array of IntPoint Structure"))
  (bind _keys (`BlueprintMapLibrary.Map_Keys` (`self.Grid Tiles Data`)))
  (for _array_element _keys
    (bind (_index _tiletype _tiletransform _tilestate _unitontile _obstacles) (break `/Game/Blueprints/Grid/F_TileData` (`BlueprintMapLibrary.Map_Find` (`self.Grid Tiles Data`) _array_element)))
    (if (`.ReturnValue` (`BlueprintMapLibrary.Map_Find` _obstacles (`local.Obstacle`)))
      (`KismetArrayLibrary.Array_Add` (`local.Obstacle Indexes`) _index)))
  (return (`local.Obstacle Indexes`)))

(fn `Get All Tiles With State`
  (params (State :type "/Game/Blueprints/Grid/Enum_TileStates Enum" :default "NewEnumerator0"))
  (returns (Indexe :type "Array of IntPoint Structure"))
  (locals (RET :type "Array of IntPoint Structure"))
  (return (`.IntPointArray_8_A4A5DA25498C5D4C2CA28DB0D7A524DF` (break `/Game/Blueprints/Grid/F_IntPointArray` (`BlueprintMapLibrary.Map_Find` (`self.Tile State To Indexes`) State)))))

(fn `Get Cursor Location on Grid`
  (params (PlayerIndex :type Integer) (`Trace For Ground` :type Boolean) (`Trace for Empty Space` :type Boolean))
  (returns (Location :type "Vector Structure"))
  (bind (_hitresult _returnvalue) (`PlayerController.GetHitResultUnderCursorByChannel` (`GameplayStatics.GetPlayerController` (`local.PlayerIndex`)) "TraceTypeQuery3" true))
  (bind (_worldlocation _worlddirection) (`PlayerController.DeprojectMousePositionToWorld` (`GameplayStatics.GetPlayerController` (`local.PlayerIndex`))))
  (bind (_hitresult_2 _returnvalue_2) (`PlayerController.GetHitResultUnderCursorByChannel` (`GameplayStatics.GetPlayerController` (`local.PlayerIndex`)) "TraceTypeQuery4" true))
  (`|ExecutionSequence`
    (:`then_0`
      (`|ExecutionSequence`
        (:`then_0`
          (if _returnvalue_2
            (return (`.Location` (`GameplayStatics.BreakHitResult` _hitresult_2)))))
        (:`then_1`
          (if (`local.Trace For Ground`)
            (if _returnvalue
              (return (`.Location` (`GameplayStatics.BreakHitResult` _hitresult))))))
        (:`then_2`
          (if (`local.Trace for Empty Space`)
            (return (`.Intersection` (`KismetMathLibrary.LinePlaneIntersection` _worldlocation (+ _worldlocation (* _worlddirection 1000000000.0)) (`KismetMathLibrary.MakePlaneFromPointAndNormal` (`self.Center Location`)))))))))
    (:`then_1`
      (return (-999.0 -999.0 -999.0)))))

(fn `Get Tile Index from Location`
  (params (Location :type "Vector Structure"))
  (returns (Index :type "IntPoint Structure"))
  (locals (`Location on Grid` :type "Vector Structure") (`Snaped Location` :type "Vector2D Structure") (`Temp Vector` :type "Vector2D Structure"))
  (bind (_temp_vector_x _temp_vector_y) (`KismetMathLibrary.BreakVector2D` (`local.Temp Vector`)))
  (bind _temp_vector_x_2 (`KismetMathLibrary.BreakVector2D` (`local.Temp Vector`)))
  (bind (_temp_vector_x_3 _temp_vector_y_2) (`KismetMathLibrary.BreakVector2D` (`local.Temp Vector`)))
  (bind _output_get (set `local.Location on Grid` (- Location (`self.Grid Origin Position`))))
  (if (!= _output_get (-999.0 -999.0 -999.0) :`ErrorTolerance` 0.001)
    (switch `/Game/Blueprints/Grid/Enum_GridShapeData` (`self.Tile Shape`)
      (:`NewEnumerator0`
        (return (make `IntPoint` -999 -999)))
      (:`NewEnumerator1`
        (bind _output_get_2 (set `local.Snaped Location` (`KismetMathLibrary.Conv_VectorToVector2D` (`/Game/Blueprints/Core/Utility/BPFL_Utility.Snap Vector to Vector` (`local.Location on Grid`) (`self.Tile Size`)))))
        (return (`KismetMathLibrary.Conv_Vector2DToIntPoint` (/ _output_get_2 (`KismetMathLibrary.Conv_VectorToVector2D` (`self.Tile Size`))))))
      (:`NewEnumerator2`
        (set `local.Snaped Location` (`KismetMathLibrary.Conv_VectorToVector2D` (`/Game/Blueprints/Core/Utility/BPFL_Utility.Snap Vector to Vector` (* (`local.Location on Grid`) (1.0 2.0 1.0)) (* (`self.Tile Size`) (0.75 0.25 1.0)))))
        (set `local.Temp Vector` (/ (`local.Snaped Location`) (* (`KismetMathLibrary.Conv_VectorToVector2D` (`self.Tile Size`)) (0.75 1.0))))
        (if (`/Game/Blueprints/Core/Utility/BPFL_Utility.Is Float Even` _temp_vector_x_2)
          (return (make `IntPoint` (`KismetMathLibrary.FTrunc` _temp_vector_x_3) (`KismetMathLibrary.FTrunc` (* (`KismetMathLibrary.Round` (/ _temp_vector_y_2 2.0)) 2.0))))
          (else
            (return (make `IntPoint` (`KismetMathLibrary.FTrunc` _temp_vector_x) (`KismetMathLibrary.FTrunc` (+ (* (`KismetMathLibrary.FFloor` (/ _temp_vector_y 2.0)) 2.0) 1.0))))))))
    (else
      (return (make `IntPoint` -999 -999)))))

(fn `Get Tile Size from Grid Shape`
  (params (Enumerator :type "/Game/Blueprints/Grid/Enum_GridShapeData Enum" :default "NewEnumerator0"))
  (returns (`Tile Size` :type "Vector Structure"))
  (bind _returnvalue (`|GetDataTableRow` "/Game/Blueprints/Grid/DT_GridShapeData.DT_GridShapeData" (`KismetStringLibrary.Conv_StringToName` (`|GetEnumeratorNameAsString` Enumerator)))
    (:`then`
      (return (`.MeshSize_4_D0DCCCA64761516B3CECF79D72BD4D1B` (break `/Game/Blueprints/Grid/F_GridShapeData` _returnvalue))))
    (:`RowNotFound`
      (return (0.0 0.0 0.0)))))

(fn `Get Tile Transform Scale`
  (returns (`Tile Transform Scale` :type "Vector Structure"))
  (return (/ (`self.Tile Size`) (`.MeshSize_4_D0DCCCA64761516B3CECF79D72BD4D1B` (break `/Game/Blueprints/Grid/F_GridShapeData` (`self.Out Row`))))))

(fn `Get Tile Under Cursor`
  (params (PlayerIndex :type Integer) (`Trace For Ground` :type Boolean) (`Trace for Empty Space` :type Boolean))
  (returns (Index :type "IntPoint Structure"))
  (bind _location (`self.Get Cursor Location on Grid` PlayerIndex `Trace For Ground` `Trace for Empty Space`))
  (bind _index (`self.Get Tile Index from Location` _location))
  (return _index))

(fn `Is Index Valid`
  (params (Index :type "IntPoint Structure"))
  (returns (`Is Valid` :type Boolean))
  (return (`BlueprintMapLibrary.Map_Contains` (`self.Grid Tiles Data`) Index)))

(fn `Is Tile Walkable`
  (params (Index :type "IntPoint Structure"))
  (returns (`Is Empty Space` :type Boolean))
  (return (`/Game/Blueprints/Core/Utility/BPFL_Utility.Is Tile Type Walkable` (`.TileType_7_99A5401643D0FD504FC2D2B4806678DB` (break `/Game/Blueprints/Grid/F_TileData` (`BlueprintMapLibrary.Map_Find` (`self.Grid Tiles Data`) Index))))))

(fn `Remove Grid Tile`
  (params (Index :type "IntPoint Structure"))
  (bind _returnvalue (`BlueprintMapLibrary.Map_Remove` (`self.Grid Tiles Data`) Index))
  (if _returnvalue
    (`/Game/Blueprints/Grid/BP_GridVisual.Update Tile Visual` (`self.As BP Grid Visual`) (make `/Game/Blueprints/Grid/F_TileData` Index "NewEnumerator1" "0.000000,0.000000,0.000000|0.000000,0.000000,0.000000|1.000000,1.000000,1.000000" _ null))
    (`self.OnTileDataUpdated` (`local.Index`))))

(fn `Remove State from Tile`
  (params (Index :type "IntPoint Structure") (State :type "/Game/Blueprints/Grid/Enum_TileStates Enum" :default "NewEnumerator0"))
  (locals (Data :type "/Game/Blueprints/Grid/F_TileData Structure"))
  (bind _data_index (break `/Game/Blueprints/Grid/F_TileData` (`local.Data`)))
  (bind (_value _returnvalue) (`BlueprintMapLibrary.Map_Find` (`self.Grid Tiles Data`) Index))
  (if _returnvalue
    (bind _output_get (set `local.Data` _value))
    (bind _returnvalue_2 (`KismetArrayLibrary.Array_RemoveItem` (`.TileState_15_2CD077A14CF44985E0DDB1AF1B2DA5B7` (break `/Game/Blueprints/Grid/F_TileData` _output_get)) State))
    (if _returnvalue_2
      (`BlueprintMapLibrary.Map_Add` (`self.Grid Tiles Data`) _data_index (`local.Data`))
      (bind _indexe (`self.Get All Tiles With State` (`local.State`)))
      (`KismetArrayLibrary.Array_RemoveItem` _indexe (`local.Index`))
      (`BlueprintMapLibrary.Map_Add` (`self.Tile State To Indexes`) (`local.State`) (make `/Game/Blueprints/Grid/F_IntPointArray` _indexe))
      (`/Game/Blueprints/Grid/BP_GridVisual.Update Tile Visual` (`self.As BP Grid Visual`) (`local.Data`))
      (`self.On Tile State Updated` (`local.Index`)))))

(fn `Spawn Grid`
  (params (`Tile Count` :type "IntPoint Structure") (`Tile Type` :type "/Game/Blueprints/Grid/Enum_GridShapeData Enum" :default "NewEnumerator0") (`Center Location` :type "Vector Structure") (`Tile Size` :type "Vector Structure"))
  (locals (`X Index` :type Integer) (`Y Index` :type Integer) (`Tile Transform` :type "Transform Structure") (`Snapped Center` :type "Vector Structure" :default (0.0 0.0 0.0)))
  (bind (_tile_count_x _tile_count_y) (break `IntPoint` (`self.Tile Count`)))
  (bind (_tile_count_x_2 _tile_count_y_2) (break `IntPoint` (`self.Tile Count`)))
  (bind _tile_count_x_3 (break `IntPoint` (`self.Tile Count`)))
  (set `self.Tile Count` `Tile Count`)
  (set `self.Tile Shape` `Tile Type`)
  (set `self.Center Location` `Center Location`)
  (set `self.Tile Size` `Tile Size`)
  (`BlueprintMapLibrary.Map_Clear` (`self.Grid Tiles Data`))
  (`self.Destroy Grid`)
  (bind _returnvalue (`|GetDataTableRow` "/Game/Blueprints/Grid/DT_GridShapeData.DT_GridShapeData" (`KismetStringLibrary.Conv_StringToName` (`|GetEnumeratorNameAsString` (`self.Tile Shape`))))
    (:`then`
      (set `self.Out Row` _returnvalue)
      (`/Game/Blueprints/Grid/BP_GridVisual.Initialize Grid Visual` (`self.As BP Grid Visual`) self)
      (bind (_origin _center) (`self.Calculate Origin Point`))
      (set `self.Center Location` _center)
      (set `self.Grid Origin Position` _origin)
      (for _index (range _tile_count_x_3)
        (set `local.X Index` _index)
        (switch `/Game/Blueprints/Grid/Enum_GridShapeData` (`self.Tile Shape`)
          (:`NewEnumerator1`
            (for _index_2 (range _tile_count_y)
              (set `local.Y Index` _index_2)
              (bind _output_get (set `self.Index Point` (make `IntPoint` (`local.X Index`) (`local.Y Index`)) :!label _label))
              (bind (_transition _scale) (`self.Tile Transform Calculations` (`KismetMathLibrary.Conv_IntPointToVector2D` _output_get)))
              (bind _output_get_2 (set `local.Tile Transform` (`KismetMathLibrary.MakeTransform` _transition (struct) _scale)))
              (if (`self.Use Enviorment`)
                (bind (_hit_tile_type _out_location) (`self.Trace for Ground` (.location _output_get_2)))
                (`self.Add Grid Tile` (make `/Game/Blueprints/Grid/F_TileData` (`self.Index Point`) _hit_tile_type (`KismetMathLibrary.MakeTransform` _out_location (.rotation _output_get_2) (.scale _output_get_2)) _ null))
                (else
                  (`self.Add Grid Tile` (make `/Game/Blueprints/Grid/F_TileData` (`self.Index Point`) "NewEnumerator0" (`local.Tile Transform`) _ null))))
              (`self.OnGridGenerated`)))
          (:`NewEnumerator2`
            (for _index_3 (range (`KismetMathLibrary.SelectInt` 0 1 (`/Game/Blueprints/Core/Utility/BPFL_Utility.Is Int Even` (`local.X Index`))) (* _tile_count_y_2 2))
              (set `local.Y Index` _index_3)
              (`|ExecutionSequence`
                (:`then_0`
                  (goto _label))
                (:`then_1`
                  (`/Engine/EditorBlueprintResources/StandardMacros.IncrementInt` _index_3))))))))))

(fn `Tile Transform Calculations`
  (params (Index :type "Vector2D Structure"))
  (returns (Transition :type "Vector Structure") (Scale :type "Vector Structure"))
  (return (+ (* (`KismetMathLibrary.Conv_Vector2DToVector` (* Index (select `/Game/Blueprints/Grid/Enum_GridShapeData` (`self.Tile Shape`) :`NewEnumerator1` (1.0 1.0) :`NewEnumerator2` (0.75 0.5) :!type "Vector2D Structure"))) (`self.Tile Size`)) (`self.Grid Origin Position`)) (`self.Get Tile Transform Scale`)))

(fn `Trace for Ground`
  (params (Location :type "Vector Structure"))
  (returns (`Hit Tile Type` :type "/Game/Blueprints/Grid/Obstacles/Enum_TileTypes Enum") (`Out Location` :type "Vector Structure"))
  (locals (Radius :type "Float (single-precision)" :default 0.0) (Loc :type "Vector Structure") (`Ret type` :type "/Game/Blueprints/Grid/Obstacles/Enum_TileTypes Enum"))
  (bind _loc (`local.Loc`))
  (bind (_loc_x _loc_y) (`KismetMathLibrary.BreakVector` (`local.Loc`)))
  (bind (_tile_size_x _tile_size_y _tile_size_z) (`KismetMathLibrary.BreakVector` (`self.Tile Size`)))
  (set `local.Loc` Location)
  (bind _output_get (set `local.Radius` (/ _tile_size_z 2.35)))
  (bind _outhits (`KismetSystemLibrary.SphereTraceMulti` (+ _loc (0.0 0.0 100.0)) (- _loc (0.0 0.0 100.0)) _output_get "TraceTypeQuery3"))
  (if (> (`KismetArrayLibrary.Array_Length` _outhits) 0)
    (set `local.Ret type` "NewEnumerator0")
    (for _array_element _outhits
      (bind (_bblockinghit _binitialoverlap _time _distance _location _impactpoint _normal _impactnormal _physmat _hitactor) (`GameplayStatics.BreakHitResult` _array_element))
      (bind _asbp_grid_modifier (cast `/Game/Blueprints/Grid/Obstacles/BP_GridModifier` _hitactor))
      (bind _output_get_2 (set `local.Ret type` (`/Game/Blueprints/Grid/Obstacles/BP_GridModifier.Tile Type` _asbp_grid_modifier))))
    (return _output_get_2 (`KismetMathLibrary.MakeVector` _loc_x _loc_y (+ (.z _impactpoint) 0.1)))
    (else
      (return "NewEnumerator1" (`local.Loc`)))))

(fn `UserConstructionScript`
  (set `self.As BP Grid Visual` (cast `/Game/Blueprints/Grid/BP_GridVisual` (`ChildActorComponent.ChildActor` (`self.Grid Visual`)) :!pure true))
  (bind _output_get (set `self.As BP Pathfinding` (cast `/Game/Blueprints/Character/BP_Pathfinding` (`ChildActorComponent.ChildActor` (`self.ChildActor_Pathfinding`)) :!pure true)))
  (set `/Game/Blueprints/Character/BP_Pathfinding.Grid Ref` self _output_get)
  (bind _output_get_2 (set `self.As BP Pathfinding Reachables` (cast `/Game/Blueprints/Character/BP_Pathfinding` (`ChildActorComponent.ChildActor` (`self.ChildActor_Pathfindiing Reachables`)) :!pure true)))
  (set `/Game/Blueprints/Character/BP_Pathfinding.Grid Ref` self _output_get_2)
  ;[0 0 0] Connect to debug the grid in editor without starting the game
  (set `self.Tile Size` (`self.Get Tile Size from Grid Shape` (`self.Tile Shape`)))
  (`self.Spawn Grid` (`self.Tile Count`) (`self.Tile Shape`) (`self.K2_GetActorLocation`) (`self.Tile Size`)))